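; Office desk actor that plays visual upgrade effects for the desk and for its computer set (PC, keyboard, mouse, monitor).
; DeskUpgradeEffect and ComputerUpgradeEffect each wait, then a timeline drives the UpgradeScalar material parameter.
; A Delay off that timeline's Update activates UpgradeEffect, swaps in upgraded materials and starts a second timeline driving the same parameter on them.
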(event Custom|DeskUpgradeEffect
  ;[0.7765 0.01177 1] Desk Upgrade Effect
  (Utilities|FlowControl|Delay 2.0)
  (bind _newtrack_0 (Timeline|Timeline PlayFromStart)
    (:Update
      (Rendering|Material|SetScalarParameterValueonMaterials (Variables|Default|GetOfficeDesk) "UpgradeScalar" _newtrack_0)
      (Utilities|FlowControl|Delay 0.5)
      (Components|Activation|SetActive (Variables|Default|GetUpgradeEffect) true false)
      (Rendering|Material|SetMaterial (Variables|Default|GetOfficeDesk) 0 "/Game/GameJamContent/Assets/Office/Props/Textures/Desk/MMI_DeskUpgrade1.MMI_DeskUpgrade1")
      (bind _newtrack_0_2 (Timeline|Timeline_0 PlayFromStart)
        (:Update
          (Rendering|Material|SetScalarParameterValueonMaterials (Variables|Default|GetOfficeDesk) "UpgradeScalar" _newtrack_0_2))))))

(event Custom|ComputerUpgradeEffect
  (bind _mouse (Variables|Default|GetMouse))
  (bind _monitor (Variables|Default|GetMonitor))
  (bind _pc (Variables|Default|GetPC))
  (bind _keyboard (Variables|Default|GetKeyboard))
  (bind _array (Utilities|Array|MakeArray _pc _keyboard _mouse _monitor))
  ;[0.7765 0.01177 1] Computor Upgrade Effect
  (Utilities|FlowControl|Delay 2.0)
  (bind _newtrack_0 (Timeline|Timeline_1 PlayFromStart)
    (:Update
      (Rendering|Material|SetScalarParameterValueonMaterials _array "UpgradeScalar" _newtrack_0)
      (Utilities|FlowControl|Delay 0.5)
      (Components|Activation|SetActive (Variables|Default|GetUpgradeEffect) true false)
      (CallFunction|SetComputorMaterials)
      (bind _newtrack_0_2 (Timeline|Timeline_2 PlayFromStart)
        (:Update
          (Rendering|Material|SetScalarParameterValueonMaterials _array "UpgradeScalar" _newtrack_0_2))))))

(event Custom|SetComputorMaterials
  ;[0.7765 0.01177 1] Computor Upgrade Effect
  (Rendering|Material|SetMaterial (Variables|Default|GetPC) 0 "/Game/GameJamContent/Assets/Office/Props/Textures/PC/MMI_PCUpgrade1.MMI_PCUpgrade1")
  (Rendering|Material|SetMaterial (Variables|Default|GetKeyboard) 0 "/Game/GameJamContent/Assets/Office/Props/Textures/Keyboard/MMI_KeyboardUpgrade1.MMI_KeyboardUpgrade1")
  (Rendering|Material|SetMaterial (Variables|Default|GetMouse) 0 "/Game/GameJamContent/Assets/Office/Props/Textures/Mouse/MMI_MouseUpgrade1.MMI_MouseUpgrade1")
  (Rendering|Material|SetMaterial (Variables|Default|GetMonitor) 0 "/Game/GameJamContent/Assets/Office/Props/Textures/Monitor/MMI_MonitorUpgrade1.MMI_MonitorUpgrade1"))

(event EventBeginPlay)

(fn ConstructionScript)