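; Standard enemy character that senses the player, attacks in melee and serves an AI controller.
; PawnSensing hearing and sight events write blackboard keys and cache the player as Target.
; AttackPlayer sphere-traces forward to deal damage, while health, healing and incoming damage forward to DamagableComponent, whose death event ragdolls the mesh, notifies the controller and spawns random embers.
; Getter and setter functions expose patrol route, ideal ranges and movement speed.
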(event OnSeePawn(PawnSensing)
  (params (Pawn :type Pawn%20Object%20Reference))
  (AI|Components|Blackboard|SetValueasBool (AI|GetBlackboard (AI|GetAIController self)) (Variables|Default|GetSeenPlayer?) true)
  (bind _asbp_third_person_character (Utilities|Casting|CastToBP_ThirdPersonCharacter (AI|Components|Blackboard|GetValueasObject (AI|GetBlackboard (AI|GetAIController self)) (Variables|Default|GetTargetName))))
  (Variables|Default|SetTarget _asbp_third_person_character))

(event OnHearNoise(PawnSensing)
  (params (Instigator :type Pawn%20Object%20Reference) (Location :type Vector%20%28by%20ref%29 :default "0, 0, 0") (Volume :type Float%20%28single-precision%29))
  (bind _self self)
  (AI|Components|Blackboard|SetValueasBool (AI|GetBlackboard (AI|GetAIController _self)) (Variables|Default|GetHeardPlayer?) true)
  (AI|Components|Blackboard|SetValueasVector (AI|GetBlackboard (AI|GetAIController _self)) (Variables|Default|GetSoundLocation) Location)
  (bind _asbp_third_person_character (Utilities|Casting|CastToBP_ThirdPersonCharacter (AI|Components|Blackboard|GetValueasObject (AI|GetBlackboard (AI|GetAIController self)) (Variables|Default|GetTargetName))))
  (Variables|Default|SetTarget _asbp_third_person_character))

(event Custom|AttackPlayer
  (bind _returnvalue (Transformation|GetActorLocation))
  (bind (_outhit _returnvalue_2) (Collision|SphereTraceForObjects _returnvalue (+ _returnvalue (* (Math|Vector|GetForwardVector (Transformation|GetActorRotation)) 2.5e+02)) 1.2e+02 (Utilities|Array|MakeArray "ObjectTypeQuery3") false 0 "None"))
  (if _returnvalue_2
    (Class|BPIDamageable|TakeDamage(Message) (.HitActor (Collision|BreakHitResult _outhit)) (Utilities|Struct|MakeS_DamageInfo 1e+01 "NewEnumerator1" "NewEnumerator1" false))))

(event Custom|OnDeath
  (bind _mesh (Variables|Character|GetMesh))
  (Physics|SetSimulatePhysics _mesh true)
  (Collision|SetCollisionEnabled _mesh "QueryAndPhysics")
  (bind _asai_controller (Utilities|Casting|CastToAI_Controller (Pawn|GetController)))
  (Default|Died _asai_controller)
  (for _index (range 0 (Math|Random|RandomIntegerinRange 0 4))
    (Game|SpawnActorfromClass "/Game/GameJamContent/Interactables/Dungeon/BP_Embers.BP_Embers_C" (Transformation|GetActorTransform) "Undefined" "MultiplyWithRoot" 0 0)))

(event Custom|DamageResponse
  (params (DamageResponse :type E_DamageResponse%20Enum :default "NewEnumerator0")))

(event EventBeginPlay)

(event Collision|EventActorBeginOverlap
  (params (OtherActor :type Actor%20Object%20Reference)))

(event EventTick
  (params (DeltaSeconds :type Float%20%28single-precision%29)))

(fn ConstructionScript
  (bind _damagablecomponent (Variables|Default|GetDamagableComponent))
  (EventDispatchers|BindEventtoOnDeath _damagablecomponent (EventDispatchers|CreateEvent :!event Custom|OnDeath))
  (EventDispatchers|BindEventtoOnDamageResponse _damagablecomponent (EventDispatchers|CreateEvent :!event Custom|DamageResponse)))

(fn GetCurrentHealth
  (return (Variables|/Game/GameJamContent/DamageSystem/DamagableComponent.DamagableComponent_C|GetHealth (Variables|Default|GetDamagableComponent))))

(fn GetMaxHealth
  (return (Variables|/Game/GameJamContent/DamageSystem/DamagableComponent.DamagableComponent_C|GetMaxHealth (Variables|Default|GetDamagableComponent))))

(fn GetRoamRoute
  (return (Variables|Default|GetPatrolRoute)))

(fn Heal
  (params (Amount :type Float%20%28double-precision%29))
  (bind _newhealth (Default|Heal (Variables|Default|GetDamagableComponent) Amount))
  (return _newhealth))

(fn IdealRange
  (return 1e+02 3e+02))

(fn SetMoveSpeed
  (params (NewParam :type MoveSpeed%20Enum :default "NewEnumerator0"))
  (bind _output_get (Variables|/Script/Engine.CharacterMovementComponent|SetMaxWalkSpeed (Variables|Character|GetCharacterMovement) (Utilities|Select :Index NewParam :NewEnumerator0 0.0 :NewEnumerator1 1.5e+02 :NewEnumerator2 3e+02 :NewEnumerator3 6e+02)))
  (return _output_get))

(fn TakeDamage
  (params (DamageInfo :type S%20Damage%20Info%20Structure))
  (bind _wasdamaged (Default|TakeDamage (Variables|Default|GetDamagableComponent) DamageInfo))
  (return _wasdamaged))