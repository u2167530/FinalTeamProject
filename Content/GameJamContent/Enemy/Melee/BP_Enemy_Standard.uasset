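; Standard melee enemy, a child Blueprint that adds attack, hit reaction and death behavior and supplies its own attack and defend radii.
; Attacks play a montage and call the parent attack after a short delay, unless the enemy has died.
; TakeDamage routes through DamagableComponent, showing damage and applying knockback on success.
; Death triggers hitstop by zeroing CustomTimeDilation until a timer restores it, plays a montage, then freezes and destroys the actor.
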(event Custom|MeleeAttack
  ;[0.07477 1 0] This event plays the attack animation
)

(event EventBeginPlay
  (|CallParentFunction))

(event Collision|EventActorBeginOverlap
  (params (OtherActor :type Actor%20Object%20Reference))
  (|CallParentFunction OtherActor) ; This node is disabled and will not be called.\nDrag off pins to build functionality.
)

(event EventTick
  (params (DeltaSeconds :type Float%20%28single-precision%29))
  (|CallParentFunction DeltaSeconds) ; This node is disabled and will not be called.\nDrag off pins to build functionality.
)

(event EventAttackPlayer
  (if (not (Variables|Default|GetDied?))
    (Animation|PlayAnimMontage "/Game/GameJamContent/Enemy/Melee/LatestAnimations/Attack/AnimMon_MeleeAttack_Latest.AnimMon_MeleeAttack_Latest" 1.0 "None")
    (Utilities|FlowControl|Delay 0.6)
    (if (not (Variables|Default|GetDied?))
      (|CallParentFunction))))

(event EventOnDeath
  ;[0.2917 0.006281 0] Death
  (Variables|Default|SetDied? true)
  (Utilities|FlowControl|DelayUntilNextTick)
  (CallFunction|StartHitstop (Variables|Default|GetHitstopDuration))
  (|CallParentFunction)
  (Animation|PlayAnimMontage "/Game/GameJamContent/Enemy/Melee/LatestAnimations/Death/AnimMon_MeleeDeathLatest1.AnimMon_MeleeDeathLatest1" 1.0 "None")
  (Utilities|FlowControl|Delay 0.8)
  (Components|Activation|SetActive (Variables|Character|GetCharacterMovement) false false)
  (Variables|/Script/Engine.SkeletalMeshComponent|SetbPauseAnims (Variables|Character|GetMesh) true)
  (Utilities|FlowControl|Delay 1.0)
  (Actor|DestroyActor))

(fn ConstructionScript
  (|CallParentFunction))

(fn IdealRange
  (return 1.5e+02 3e+02))

(fn TakeDamage
  (params (DamageInfo :type S%20Damage%20Info%20Structure))
  (bind _wasdamaged (Default|TakeDamage (Variables|Default|GetDamagableComponent) DamageInfo))
  (if _wasdamaged
    (CallFunction|ShowDamage (.Amount (Utilities|Struct|BreakS_DamageInfo DamageInfo)))
    (CallFunction|KnockBack DamageInfo _wasdamaged (Variables|Default|GetKnockBackSize))
    (return false)))

(fn StartHitstop
  (params (Duration :type Float%20%28double-precision%29))
  (Variables|Default|SetCustomTimeDilation 0.0)
  (Utilities|Time|SetTimerbyFunctionName 0 "EndHitstop" Duration))

(fn EndHitstop
  (Variables|Default|SetCustomTimeDilation 1.0))