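; Projectile for the ranged enemy attack that explodes on contact and has a short fixed lifespan.
; HitBox overlaps with non-enemy "CanTakeDamage" actors, or Sphere hits on any non-enemy, trigger Explode and print the actor's name.
; Explode spawns a particle effect, enables Explosion collision, then immediately destroys the actor.
; Explosion overlaps apply damage to any "CanTakeDamage" actor, without filtering out enemies.
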(event OnComponentBeginOverlap(HitBox)
  (params (OverlappedComponent :type Primitive%20Component%20Object%20Reference) (OtherActor :type Actor%20Object%20Reference) (OtherComp :type Primitive%20Component%20Object%20Reference) (OtherBodyIndex :type Integer) (bFromSweep :type Boolean) (SweepResult :type Hit%20Result%20Structure%20%28by%20ref%29))
  (if (Actor|ActorHasTag OtherActor "CanTakeDamage")
    (if (not (Actor|ActorHasTag OtherActor "Enemy"))
      (CallFunction|Explode)
      (Development|PrintString (Utilities|GetDisplayName OtherActor)))))

(event OnComponentHit(Sphere)
  (params (HitComponent :type Primitive%20Component%20Object%20Reference) (OtherActor :type Actor%20Object%20Reference) (OtherComp :type Primitive%20Component%20Object%20Reference) (NormalImpulse :type Vector :default "0, 0, 0") (Hit :type Hit%20Result%20Structure%20%28by%20ref%29))
  (if (not (Actor|ActorHasTag OtherActor "Enemy"))
    (CallFunction|Explode)
    (Development|PrintString (Utilities|GetDisplayName OtherActor))))

(event OnComponentBeginOverlap(Explosion)
  (params (OverlappedComponent :type Primitive%20Component%20Object%20Reference) (OtherActor :type Actor%20Object%20Reference) (OtherComp :type Primitive%20Component%20Object%20Reference) (OtherBodyIndex :type Integer) (bFromSweep :type Boolean) (SweepResult :type Hit%20Result%20Structure%20%28by%20ref%29))
  (if (Actor|ActorHasTag OtherActor "CanTakeDamage")
    (Game|Damage|ApplyDamage OtherActor 1.0 0 0)))

(event Custom|Explode
  (Effects|SpawnEmitteratLocation "/Game/StarterContent/Particles/P_Explosion.P_Explosion" (Transformation|GetActorLocation))
  (Collision|SetCollisionEnabled (Variables|Default|GetExplosion) "QueryAndPhysics")
  (Actor|DestroyActor))

(event EventBeginPlay
  (Actor|SetLifeSpan 2.0))

(fn ConstructionScript)