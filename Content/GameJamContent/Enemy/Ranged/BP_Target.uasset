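; Ground telegraph for a ranged enemy's area attack that shows the danger zone, then damages what it hits.
; On spawn a vertical sphere trace snaps both markers to the ground, or destroys the actor if it finds none.
; Tick flattens the markers and scales Grow to fill the radius-sized Sphere over time T.
; When time expires, a sphere trace at the actor location sends damage once, then the actor destroys itself.
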(event Custom|Destroyed?
  (params (Valid :type Boolean))
  (Actor|DestroyActor))

(event EventBeginPlay
  (bind (_outhit _returnvalue) (Collision|SphereTraceForObjects (+ (Transformation|GetWorldLocation (Variables|Default|GetSphere)) (* (Math|Vector|MakeVector 0.0 0.0 1.0) 4e+02)) (+ (Transformation|GetWorldLocation (Variables|Default|GetSphere)) (* (Math|Vector|MakeVector 0.0 0.0 1.0) -4e+02)) 2e+01 (Utilities|Array|MakeArray "ObjectTypeQuery1" "ObjectTypeQuery2") false 0 "None"))
  (if _returnvalue
    (Transformation|SetWorldLocation (Variables|Default|GetGrow) (.ImpactPoint (Collision|BreakHitResult _outhit)) false true)
    (Transformation|SetWorldLocation (Variables|Default|GetSphere) (.ImpactPoint (Collision|BreakHitResult _outhit)) false true)
    (else
      (CallFunction|Destroyed? false))))

(event Collision|EventActorBeginOverlap
  (params (OtherActor :type Actor%20Object%20Reference)))

(event EventTick
  (params (DeltaSeconds :type Float%20%28single-precision%29))
  (bind _radius (Variables|Default|GetRadius))
  (bind _returnvalue (/ _radius 5e+01))
  (Transformation|SetWorldScale3D (Variables|Default|GetSphere) (Math|Vector|MakeVector _returnvalue _returnvalue 0.0))
  (bind _output_get (Variables|Default|SetTimer (+ (Variables|Default|GetTimer) DeltaSeconds)))
  (Transformation|SetWorldScale3D (Variables|Default|GetGrow) (Math|Vector|MakeVector (* (/ _output_get (Variables|Default|Gett)) (.x (Transformation|GetWorldScale (Variables|Default|GetSphere)))) (* (/ _output_get (Variables|Default|Gett)) (.x (Transformation|GetWorldScale (Variables|Default|GetSphere)))) 0.0))
  (if (> (Variables|Default|GetTimer) (Variables|Default|Gett))
    (Utilities|FlowControl|DoOnce false
      (:Completed
        (bind (_hitactor _location) (|CalAttackHit_2_2)
          (:then
            (Class|BPIDamageable|TakeDamage(Message) _hitactor (Utilities|Struct|MakeS_DamageInfo 1e+01 (Variables|Default|GetDamage%20Type) "NewEnumerator1" (Variables|Default|GetShould%20Damage%20Invincible) _location (Variables|Default|GetKnock%20Up%20Dur))))
          (:NoHit
            _))
        (CallFunction|Destroyed? true)))))

(fn ConstructionScript)