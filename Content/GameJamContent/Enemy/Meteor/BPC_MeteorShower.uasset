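; Actor component that runs a meteor shower around the player character while activated.
; A custom WhileWithDelay macro repeats CallMeteor at a set Rate; deactivation breaks the loop.
; Each call leads the player's position using velocity plus random scatter, spawning a ground target marker and a meteor high above the player aimed at it.
; It binds to BP_PauseDispatcher, retrying until found, to halt and resume the shower.
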(event Custom|DeactivateShower
  (Variables|Default|SetActive? false)
  (Utilities|WhilewithDelay (not (Variables|Default|GetPauseD?)) (Variables|Default|GetRate)) ; enters at Break
)

(event Custom|ActivateShower
  (Variables|Default|SetActive? true)
  (Utilities|FlowControl|Delay 2.0)
  (Utilities|WhilewithDelay (not (Variables|Default|GetPauseD?)) (Variables|Default|GetRate)
    (:LoopBody
      (CallFunction|CallMeteor))))

(event Custom|Pause
  (Variables|Default|SetPauseD? true))

(event Custom|Unpause
  (Variables|Default|SetPauseD? false)
  (if (Variables|Default|GetActive?)
    (Utilities|FlowControl|Delay 2.0)
    (Utilities|WhilewithDelay (not (Variables|Default|GetPauseD?)) (Variables|Default|GetRate)
      (:LoopBody
        (CallFunction|CallMeteor)))))

(event EventBeginPlay
  (bind _asbp_third_person_character (Utilities|Casting|CastToBP_ThirdPersonCharacter (Game|GetPlayerCharacter 0)))
  (Variables|Default|SetAs%20BP%20Third%20Person%20Character _asbp_third_person_character)
  (bind _returnvalue (Actor|GetActorOfClass "/Game/GameJamContent/PauseBP/BP_PauseDispatcher.BP_PauseDispatcher_C" :!label _label))
  (Utilities|IsValid _returnvalue
    (:Is%20Valid
      (Variables|Default|SetpauseVar _returnvalue)
      (EventDispatchers|BindEventtoPause _returnvalue (delegate Custom|Pause))
      (EventDispatchers|BindEventtoUnpause _returnvalue (delegate Custom|Unpause)))
    (:Is%20Not%20Valid
      (Utilities|FlowControl|Delay 5.0)
      (goto _label))))

(event EventTick
  (params (DeltaSeconds :type Float%20%28single-precision%29)))

(fn CallMeteor
  (bind _as_bp_third_person_character (Variables|Default|GetAs%20BP%20Third%20Person%20Character))
  (bind _as_bp_third_person_character_2 (Variables|Default|GetAs%20BP%20Third%20Person%20Character))
  (bind _returnvalue (Transformation|GetActorLocation _as_bp_third_person_character))
  (bind _charactermovement (Variables|/Script/Engine.Character|GetCharacterMovement _as_bp_third_person_character))
  (bind _capsulecomponent (Variables|/Script/Engine.Character|GetCapsuleComponent _as_bp_third_person_character))
  (bind _charactermovement_2 (Variables|/Script/Engine.Character|GetCharacterMovement _as_bp_third_person_character_2))
  (bind _returnvalue_2 (Class|CharacterMovementComponent|GetLastUpdateLocation _charactermovement_2))
  (bind _returnvalue_3 (Pawn|Components|CharacterMovement|GetLastUpdateVelocity _charactermovement))
  (bind (_x _y _z) (Math|Vector|BreakVector _returnvalue_2))
  (Development|PrintString "called")
  (bind _output_get (LocalVariables|SetTargetLocation (Math|Vector|MakeVector (+ (+ (/ (.x _returnvalue_3) 3.0) (.x _returnvalue)) (Math|Random|RandomFloatinRange -6e+02 6e+02)) (+ (+ (/ (.y _returnvalue_3) 3.0) (.y _returnvalue)) (Math|Random|RandomFloatinRange -6e+02 6e+02)) (- (.z (Transformation|GetWorldLocation _capsulecomponent)) (Variables|/Script/Engine.CapsuleComponent|GetCapsuleHalfHeight _capsulecomponent)))))
  (Game|SpawnActorfromClass "/Game/GameJamContent/Enemy/Meteor/BP_Target_Meteor.BP_Target_Meteor_C" (Math|Conversions|ToTransform(Vector) _output_get) "AlwaysSpawn" "MultiplyWithRoot" 0 (Variables|Default|GetpauseVar) 1.2 2e+02 0)
  (Game|SpawnActorfromClass "/Game/GameJamContent/Enemy/Meteor/Meteor.Meteor_C" (Math|Conversions|ToTransform(Vector) (Math|Vector|MakeVector _x _y (+ _z 4e+03))) "AlwaysSpawn" "MultiplyWithRoot" 0 (LocalVariables|GetTargetLocation) 1.2 0))