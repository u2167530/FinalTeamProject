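; Meteor enemy target Blueprint that extends a parent class with item drops and pause-triggered removal.
; On BeginPlay it binds its Destroy event to the Pause event, and Destroy goes straight to the parent's destruction logic without drops.
; The overridden Destroyed event has DropableComponent spawn drops only when flagged Valid, then joins that same parent call.
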(event Custom|Destroy
  (|CallParentFunction (stale EventDestroyed? Valid)))

(event EventBeginPlay
  (|CallParentFunction)
  (EventDispatchers|BindEventtoPause (Variables|Default|GetPause) (delegate Custom|Destroy)))

(event Collision|EventActorBeginOverlap
  (params (OtherActor :type Actor%20Object%20Reference))
  (|CallParentFunction OtherActor) ; This node is disabled and will not be called.\nDrag off pins to build functionality.
)

(event EventTick
  (params (DeltaSeconds :type Float%20%28single-precision%29))
  (|CallParentFunction DeltaSeconds) ; This node is disabled and will not be called.\nDrag off pins to build functionality.
)

(event EventDestroyed?
  (params (Valid :type Boolean))
  (if Valid
    (Default|Drops (Variables|Default|GetDropableComponent) self))
  (|CallParentFunction Valid))

(fn ConstructionScript
  (|CallParentFunction))