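; BP_TargetShield is an enemy shield actor that plays slam effects as feedback, likely for a landing.
; On BeginPlay, after a short delay, it spawns BP_ShieldSlamVFX at a marker component and plays a distance-limited world camera shake.
; On Tick, once Timer passes T, a DoOnce plays the boss landing sound and spawns a second slam VFX below the actor.
; This graph never updates Timer itself.
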(event EventBeginPlay
  (|CallParentFunction)
  (Utilities|FlowControl|Delay 1.7)
  (Game|SpawnActorfromClass "/Game/GameJamContent/Effects/ShieldSlam/BP_ShieldSlamVFX.BP_ShieldSlamVFX_C" (Math|Transform|MakeTransform (Transformation|GetWorldLocation (Variables|Default|GetShieldSlamVFXLoc)) "0, 0, 0" "1.000000,1.000000,1.000000") "AlwaysSpawn" "MultiplyWithRoot" 0 0)
  (Camera|PlayWorldCameraShake "/Game/GameJamContent/Effects/CameraShake/BP_CameraShake.BP_CameraShake_C" (Transformation|GetActorLocation) 0.0 1e+03 0.0 true))

(event Collision|EventActorBeginOverlap
  (params (OtherActor :type Actor%20Object%20Reference))
  (|CallParentFunction OtherActor) ; This node is disabled and will not be called.\nDrag off pins to build functionality.
)

(event EventTick
  (params (DeltaSeconds :type Float%20%28single-precision%29))
  (bind _returnvalue (Transformation|GetActorLocation))
  (|CallParentFunction DeltaSeconds)
  (if (> (Variables|Default|GetTimer) (Variables|Default|Gett))
    (Utilities|FlowControl|DoOnce false
      (:Completed
        (Audio|PlaySound2D "/Game/GameJamContent/Sounds/Sound_Design/Beings/Enemy/Shield/Land/BossLand_Cue.BossLand_Cue" 1.0 1.0 0.0 0 0)
        (Game|SpawnActorfromClass "/Game/GameJamContent/Effects/ShieldSlam/BP_ShieldSlamVFX.BP_ShieldSlamVFX_C" (Math|Transform|MakeTransform (Math|Vector|MakeVector (.x _returnvalue) (.y _returnvalue) (- (.z _returnvalue) 2.5e+02)) "0, 0, 0" "1.000000,1.000000,1.000000") "AlwaysSpawn" "MultiplyWithRoot" 0 0)))))

(fn ConstructionScript
  (|CallParentFunction))