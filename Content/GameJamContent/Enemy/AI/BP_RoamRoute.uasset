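; BP_RoamRoute is a spline-based patrol route, filed with the enemy AI assets, that tracks a current waypoint along its Spline.
; IncrementRoute steps Index by Direction and flips Direction at the first and last spline points, so the route runs back and forth rather than looping.
; GetSplinePointWorld returns the world-space location of the spline point at the current Index.
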(event Custom|IncrementRoute
  (bind _output_get (Variables|Default|SetIndex (+ (Variables|Default|GetIndex) (Variables|Default|GetDirection))))
  (if (== _output_get (- (Spline|GetNumberOfSplinePoints (Variables|Default|GetSpline)) 1))
    (Variables|Default|SetDirection -1)
    (elif (== (Variables|Default|GetIndex) 0)
      (Variables|Default|SetDirection 1))))

(fn ConstructionScript)

(fn GetSplinePointWorld
  (return (Spline|GetLocationatSplinePoint (Variables|Default|GetSpline) (Variables|Default|GetIndex) "World")))