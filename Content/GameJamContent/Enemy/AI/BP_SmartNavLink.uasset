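; Smart nav link that makes BP_Enemy1 jump to the link's destination when it reaches the link.
; On arrival it halts the enemy, pauses its AI logic, zeroes braking friction and launches it.
; Velocity derives the launch vector with a fixed-angle projectile formula from distance, height difference and gravity.
; A delayed loop polls IsFalling, then restores friction, stops movement and restarts AI logic after a short pause.
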(event EventBeginPlay)

(event Collision|EventActorBeginOverlap
  (params (OtherActor :type Actor%20Object%20Reference)))

(event EventTick
  (params (DeltaSeconds :type Float%20%28single-precision%29)))

(event EventSmartLinkReached
  (params (Agent :type Actor%20Object%20Reference) (Destination :type Vector%20%28by%20ref%29 :default "0, 0, 0"))
  (bind (_x _y _z) (Class|KismetMathLibrary|BreakVector3f Destination))
  (bind _asbp_enemy_1 (Utilities|Casting|CastToBP_Enemy1 Agent))
  (Variables|Default|SetBraking%20Friction (Variables|/Script/Engine.CharacterMovementComponent|GetBrakingFriction (Variables|/Script/Engine.Character|GetCharacterMovement _asbp_enemy_1)))
  (Components|Movement|StopMovementImmediately (Variables|/Script/Engine.Character|GetCharacterMovement _asbp_enemy_1))
  (AI|Logic|StopLogic (Variables|/Script/AIModule.AIController|GetBrainComponent (AI|GetAIController _asbp_enemy_1)) "")
  (Utilities|FlowControl|Delay 0.2)
  (Variables|/Script/Engine.CharacterMovementComponent|SetBrakingFriction (Variables|/Script/Engine.Character|GetCharacterMovement _asbp_enemy_1) 0.0)
  (Variables|Default|Setgravity (Components|Movement|GetGravityZ (Variables|/Script/Engine.Character|GetCharacterMovement _asbp_enemy_1)))
  (bind (_velocity_x _velocity_y _velocity_z) (Utilities|Velocity (.x (Transformation|GetActorLocation _asbp_enemy_1)) (.y (Transformation|GetActorLocation _asbp_enemy_1)) (.z (Transformation|GetActorLocation _asbp_enemy_1)) _x _y _z))
  (Character|LaunchCharacter _asbp_enemy_1 (Math|Vector|MakeVector _velocity_x _velocity_y _velocity_z) true true)
  (Utilities|FlowControl|Delay 0.1)
  (Utilities|WhilewithDelay (AI|Components|NavMovement|IsFalling (Variables|/Script/Engine.Character|GetCharacterMovement _asbp_enemy_1)) (/ (Utilities|Time|GetWorldDeltaSeconds) 1e+01)
    (:Completed
      _)
    (:Fail
      _))
  (Variables|/Script/Engine.CharacterMovementComponent|SetBrakingFriction (Variables|/Script/Engine.Character|GetCharacterMovement _asbp_enemy_1) (Variables|Default|GetBraking%20Friction))
  (Components|Movement|StopMovementImmediately (Variables|/Script/Engine.Character|GetCharacterMovement _asbp_enemy_1))
  (Utilities|FlowControl|Delay 0.2)
  (Class|BrainComponent|RestartLogic (Variables|/Script/AIModule.AIController|GetBrainComponent (AI|GetAIController _asbp_enemy_1))))

(fn ConstructionScript)