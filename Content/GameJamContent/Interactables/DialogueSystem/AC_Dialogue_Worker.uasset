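; Dialogue component for worker NPCs in the game, overriding a parent Dialogue function with short office small-talk lines.
; DialogueTreeIndex selects one of several conversations, most being a single line that then clears progress and fades out.
; One branch offers reply options, where only the encouraging reply is wired: the worker thanks the player and sends a minigame happiness bonus before closing.
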(fn Dialogue
  (|CallParentFunction)
  (switch int (Variables|Default|GetDialogueTreeIndex)
    (:0
      (CallFunction|AddDialogue (Variables|Default|GetSpeakerName) "Thanks for the coffee" (Utilities|Array|MakeArray))
      (CallFunction|ClearDialogueProgress)
      (CallFunction|FadeDialogue))
    (:1
      (bind (_state _optionindex) (CallFunction|AddDialogue (Variables|Default|GetSpeakerName) "Work is so hard today" (Utilities|Array|MakeArray "Suck it up" "Its almost friday" "You have been doing really good work, so keep at it")))
      (switch Utilities|FlowControl|Switch|SwitchonEnum_DialogueState _state
        (:NewEnumerator0
          (switch int _optionindex
            (:2
              (CallFunction|AddDialogue (Variables|Default|GetSpeakerName) "Thank you" (Utilities|Array|MakeArray))
              (Class|BPiWorker|ReceiveMinigameBonus(Message) (Variables|Default|GetSpeakerRef) 0.1 "NewEnumerator3")
              (CallFunction|ClearDialogueProgress)
              (CallFunction|FadeDialogue))))))
    (:2
      (CallFunction|AddDialogue (Variables|Default|GetSpeakerName) "I need some coffee" (Utilities|Array|MakeArray))
      (CallFunction|ClearDialogueProgress)
      (CallFunction|FadeDialogue))
    (:3
      (CallFunction|AddDialogue (Variables|Default|GetSpeakerName) "The weather is nice today" (Utilities|Array|MakeArray))
      (CallFunction|ClearDialogueProgress)
      (CallFunction|FadeDialogue))
    (:4
      (CallFunction|AddDialogue (Variables|Default|GetSpeakerName) "Hey Boss, How are you doing?" (Utilities|Array|MakeArray))
      (CallFunction|ClearDialogueProgress)
      (CallFunction|FadeDialogue))))