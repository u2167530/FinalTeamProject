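; Dialogue component for the Fire God NPC, who offers a spin-the-wheel gamble that grants extra embers at the cost of higher difficulty.
; It overrides Dialogue, switching on DialogueTreeIndex between an intro, the first spin offer, and a respin offer showing rolls left and a bonus that doubles per spin.
; Accepting increments WheelsSpun, closes the conversation and opens the BPW_DNGWheel widget, with spins capped at three.
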(fn Dialogue
  (bind _wheelsspun (Variables|Default|GetWheelsSpun))
  (|CallParentFunction)
  (switch int (Variables|Default|GetDialogueTreeIndex)
    (:0
      (bind (_state _optionindex) (CallFunction|AddDialogue "FireGod" "Hi im the fire god, you can come here to spin the wheel for extra embers however the effects increase the diffculty." (Utilities|Array|MakeArray "Continue")))
      (switch Utilities|FlowControl|Switch|SwitchonEnum_DialogueState _state
        (:NewEnumerator0
          (switch int _optionindex
            (:0
              (bind (_state_2 _optionindex_2) (CallFunction|AddDialogue "FireGod" (Utilities|Text|FormatText "Do you want to spin the wheel ({rolls} rolls left)(Current bonus: 0)" (- 3 (Variables|Default|GetWheelsSpun))) (Utilities|Array|MakeArray "Yes" "No") :!label _label))
              (switch Utilities|FlowControl|Switch|SwitchonEnum_DialogueState _state_2
                (:NewEnumerator0
                  (switch int _optionindex_2
                    (:0
                      (CallFunction|ClearDialogueProgress)
                      (Math|Integer|IncrementInt (Variables|Default|GetWheelsSpun)
                        (:%20%20
                          (CallFunction|CloseConversation)
                          (bind _returnvalue (UserInterface|CreateWidget "/Game/GameJamContent/Interactables/Dungeon/UI/BPW_DNGWheel.BPW_DNGWheel_C" 0 self))
                          (UserInterface|Viewport|AddtoViewport _returnvalue 0)
                          (CallFunction|SetDialogueTreeIndex 2))))
                    (:1
                      (CallFunction|ClearDialogueProgress)
                      (CallFunction|SetDialogueTreeIndex 1)
                      (CallFunction|CloseConversation))))))))))
    (:1
      (goto _label))
    (:2
      (if (>= (Variables|Default|GetWheelsSpun) 3)
        (bind (_state_3 _optionindex_3) (CallFunction|AddDialogue "FireGod" (Utilities|Text|FormatText "No more rerolls left (Current bonus: {bonus})" (* (Math|Float|Power 2.0 (Math|Conversions|ToFloat(Integer) (Variables|Default|GetWheelsSpun))) 25.0)) (Utilities|Array|MakeArray "Continue")))
        (switch Utilities|FlowControl|Switch|SwitchonEnum_DialogueState _state_3
          (:NewEnumerator0
            (switch int _optionindex_3
              (:0
                (CallFunction|CloseConversation)
                (CallFunction|SetDialogueTreeIndex 2)))))
        (else
          (bind (_state_4 _optionindex_4) (CallFunction|AddDialogue "FireGod" (Utilities|Text|FormatText "Do you want to spin the wheel again ({rolls} rolls left)(Current bonus: {bonus})" (- 3 _wheelsspun) (* (Math|Float|Power 2.0 (Math|Conversions|ToFloat(Integer) _wheelsspun)) 25.0)) (Utilities|Array|MakeArray "Yes" "No")))
          (switch Utilities|FlowControl|Switch|SwitchonEnum_DialogueState _state_4
            (:NewEnumerator0
              (switch int _optionindex_4
                (:0
                  (CallFunction|ClearDialogueProgress)
                  (Math|Integer|IncrementInt (Variables|Default|GetWheelsSpun)
                    (:%20%20
                      (CallFunction|CloseConversation)
                      (bind _returnvalue_2 (UserInterface|CreateWidget "/Game/GameJamContent/Interactables/Dungeon/UI/BPW_DNGWheel.BPW_DNGWheel_C" 0 self))
                      (UserInterface|Viewport|AddtoViewport _returnvalue_2 0)
                      (CallFunction|SetDialogueTreeIndex 2))))
                (:1
                  (CallFunction|ClearDialogueProgress)
                  (CallFunction|SetDialogueTreeIndex 2)
                  (CallFunction|CloseConversation))))))))))