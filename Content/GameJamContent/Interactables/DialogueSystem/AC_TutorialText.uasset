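; Dialogue component holding the tutorial conversations for the office management game and its Cinder Circus combat area, voiced by Bob, the Fire God and a Tutorial speaker.
; The Dialogue override calls its parent, then switches on DialogueTreeIndex to chain AddDialogue lines through their Pass Through states.
; Branches end by closing the conversation, most also unpausing the game and clearing progress.
; The office intro also spawns a BPW_Highlight widget before its last line.
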(event EventBeginPlay)

(event EventTick
  (params (DeltaSeconds :type Float%20%28single-precision%29)))

(fn Dialogue
  (|CallParentFunction)
  (switch int (Variables|Default|GetDialogueTreeIndex)
    (:0
      (bind _state (CallFunction|AddDialogue "Bob" "Welcome back Office Manager! Your Job is to ensure that your workers are completing the contracts that come in on your PC." (Utilities|Array|MakeArray "Continue")))
      (switch Utilities|FlowControl|Switch|SwitchonEnum_DialogueState _state
        (:NewEnumerator0
          (bind _state_2 (CallFunction|AddDialogue "Bob" "If anything breaks down as you are working then you are going to have to fix it yourself, as we dont have the budget to send anyone over." (Utilities|Array|MakeArray "Continue")))
          (switch Utilities|FlowControl|Switch|SwitchonEnum_DialogueState _state_2
            (:NewEnumerator0
              (bind _state_3 (CallFunction|AddDialogue "Bob" "New quotas have been set by your boss. To not get fired make sure that you meet them." (Utilities|Array|MakeArray "Continue")))
              (switch Utilities|FlowControl|Switch|SwitchonEnum_DialogueState _state_3
                (:NewEnumerator0
                  (bind _returnvalue (UserInterface|CreateWidget "/Game/GameJamContent/Interactables/DialogueSystem/BPW_Highlight.BPW_Highlight_C"))
                  (UserInterface|Viewport|AddtoViewport _returnvalue 0)
                  (bind _state_4 (CallFunction|AddDialogue "Bob" "If you ever need to leave the office then make sure to file the form of leave. Last week you spent a lot of your time off in a \"circus\" or something, whatever that is." (Utilities|Array|MakeArray "Continue")))
                  (switch Utilities|FlowControl|Switch|SwitchonEnum_DialogueState _state_4
                    (:NewEnumerator0
                      (Game|SetGamePaused false)
                      (CallFunction|CloseConversation)
                      (CallFunction|ClearDialogueProgress))))))))))
    (:1
      (bind _state_5 (CallFunction|AddDialogue "Bob" "When a contract has started your workers happiness will decrease. If any of their happiness reaches 0 then they will stop working." (Utilities|Array|MakeArray "Continue")))
      (switch Utilities|FlowControl|Switch|SwitchonEnum_DialogueState _state_5
        (:NewEnumerator0
          (bind _state_6 (CallFunction|AddDialogue "Bob" "During a contract some workers may be interupted by office appliances breaking down. These will slow down the contract progress until they are resolved." (Utilities|Array|MakeArray "Ok")))
          (switch Utilities|FlowControl|Switch|SwitchonEnum_DialogueState _state_6
            (:NewEnumerator0
              (Game|SetGamePaused false)
              (CallFunction|CloseConversation)
              (CallFunction|ClearDialogueProgress))))))
    (:2
      (bind _state_7 (CallFunction|AddDialogue "Fire God" "Welcome to the Cinder Circus! 
You can move with WASD 
Dash with SHIFT" (Utilities|Array|MakeArray "OK")))
      (switch Utilities|FlowControl|Switch|SwitchonEnum_DialogueState _state_7
        (:NewEnumerator0
          (CallFunction|SetDialogueTreeIndex 2)
          (CallFunction|CloseConversation)
          (Game|SetGamePaused false))))
    (:3
      (bind _state_8 (CallFunction|AddDialogue "Fire God" "To defeat my minions you can LEFT CLICK to attack 
RIGHT CLICK to throw a ranged attack 
If you take damage you can press Q to heal." (Utilities|Array|MakeArray "OK")))
      (switch Utilities|FlowControl|Switch|SwitchonEnum_DialogueState _state_8
        (:NewEnumerator0
          (CallFunction|CloseConversation)
          (CallFunction|ClearDialogueProgress))))
    (:4
      (bind _state_9 (CallFunction|AddDialogue (Variables|Default|GetSpeakerName) "Hello! I'm the Fire God. If you have any free time you can enter my cinder circus and collect embers. " (Utilities|Array|MakeArray "Continue")))
      (switch Utilities|FlowControl|Switch|SwitchonEnum_DialogueState _state_9
        (:NewEnumerator0
          (bind _state_10 (CallFunction|AddDialogue (Variables|Default|GetSpeakerName) "I can exchange these embers for upgrades to your office or dungeon gear." (Utilities|Array|MakeArray "OK")))
          (switch Utilities|FlowControl|Switch|SwitchonEnum_DialogueState _state_10
            (:NewEnumerator0
              (Game|SetGamePaused false)
              (CallFunction|CloseConversation)
              (CallFunction|ClearDialogueProgress))))))
    (:5
      (bind _state_11 (CallFunction|AddDialogue "Tutorial" "This is where you select contracts to work on. You can set your workers workload which affects their happeniess during the contract." (Utilities|Array|MakeArray "OK")))
      (switch Utilities|FlowControl|Switch|SwitchonEnum_DialogueState _state_11
        (:NewEnumerator0
          (Game|SetGamePaused false)
          (CallFunction|CloseConversation)
          (CallFunction|ClearDialogueProgress))))
    (:6
      (bind _state_12 (CallFunction|AddDialogue "Tutorial" "Well done! You have finished your first contract. " (Utilities|Array|MakeArray "Continue")))
      (switch Utilities|FlowControl|Switch|SwitchonEnum_DialogueState _state_12
        (:NewEnumerator0
          (bind _state_13 (CallFunction|AddDialogue "Tutorial" "The money you have earned goes towards your current quota, make sure you have enough money by the deadline. " (Utilities|Array|MakeArray "Continue")))
          (switch Utilities|FlowControl|Switch|SwitchonEnum_DialogueState _state_13
            (:NewEnumerator0
              (bind _state_14 (CallFunction|AddDialogue "Tutorial" "Completing contracts uses up Time Tokens, when you have none left, or not enough to do any more contracts, you can click the end day button to head to the next day." (Utilities|Array|MakeArray "Ok")))
              (switch Utilities|FlowControl|Switch|SwitchonEnum_DialogueState _state_14
                (:NewEnumerator0
                  (Game|SetGamePaused false)
                  (CallFunction|CloseConversation)
                  (CallFunction|ClearDialogueProgress))))))))))