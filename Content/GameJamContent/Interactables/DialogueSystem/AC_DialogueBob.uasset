(fn Dialogue
  (|CallParentFunction)
  (switch int (Variables|Default|GetDialogueTreeIndex)
    (:Default
      (bind (_state _optionindex) (CallFunction|AddDialogue "BOB" "Hi Im Bob" (Utilities|Array|MakeArray "Hi" "Bye") :!label _label))
      (switch Utilities|FlowControl|Switch|SwitchonEnum_DialogueState _state
        (:NewEnumerator0
          (switch int _optionindex
            (:0
              (bind (_state_2 _optionindex_2) (CallFunction|AddDialogue "BOB" "Can you help me?" (Utilities|Array|MakeArray "Yes" "No")))
              (switch Utilities|FlowControl|Switch|SwitchonEnum_DialogueState _state_2
                (:NewEnumerator0
                  (switch int _optionindex_2
                    (:0
                      (bind (_state_3 _optionindex_3) (CallFunction|AddDialogue "BOB" "Thank you" (Utilities|Array|MakeArray "Continue")))
                      (switch Utilities|FlowControl|Switch|SwitchonEnum_DialogueState _state_3
                        (:NewEnumerator0
                          (switch int _optionindex_3
                            (:0
                              (CallFunction|CloseConversation false)
                              (CallFunction|SetDialogueTreeIndex 1))))))
                    (:1
                      (bind (_state_4 _optionindex_4) (CallFunction|AddDialogue "BOB" ":(" (Utilities|Array|MakeArray "Continue")))
                      (switch Utilities|FlowControl|Switch|SwitchonEnum_DialogueState _state_4
                        (:NewEnumerator0
                          (switch int _optionindex_4
                            (:0
                              (CallFunction|ClearDialogueProgress)
                              (CallFunction|CloseConversation false))))))))))
            (:1
              (CallFunction|ClearDialogueProgress)
              (CallFunction|CloseConversation false))))))
    (:0
      (goto _label))
    (:1
      (bind (_state_5 _optionindex_5) (CallFunction|AddDialogue "BOB" "Thank you" (Utilities|Array|MakeArray "Continue")))
      (switch Utilities|FlowControl|Switch|SwitchonEnum_DialogueState _state_5
        (:NewEnumerator0
          (switch int _optionindex_5
            (:0
              (CallFunction|ClearDialogueProgress)
              (CallFunction|CloseConversation false))))))))