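; Office interactable that starts a typing minigame when the player interacts with it while it is the chosen object.
; On BeginPlay it caches the widget from its TypingBox component and hands it the player character.
; Interacting freezes player movement, stores the movement component, clears the chosen flag and hides the notification and tutorial widgets.
; It then adds a new BPW_TypingBox to the viewport, passing itself and the minigame type.
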(event EventBeginPlay
  (|CallParentFunction)
  (bind _asbpw_typing_box (Utilities|Casting|CastToBPW_TypingBox (UserInterface|GetWidget (Variables|Default|GetTypingBox))))
  (Variables|Default|SetTypingBoxRef _asbpw_typing_box)
  (bind _asbp_third_person_character (Utilities|Casting|CastToBP_ThirdPersonCharacter (Game|Player|GetPlayerPawn 0)))
  (Variables|/Game/GameJamContent/Interactables/Office/UI/BPW_TypingBox.BPW_TypingBox_C|SetPlayerRef (Variables|Default|GetTypingBoxRef) _asbp_third_person_character))

(event Collision|EventActorBeginOverlap
  (params (OtherActor :type Actor%20Object%20Reference))
  (|CallParentFunction OtherActor) ; This node is disabled and will not be called.\nDrag off pins to build functionality.
)

(event EventTick
  (params (DeltaSeconds :type Float%20%28single-precision%29))
  (|CallParentFunction DeltaSeconds) ; This node is disabled and will not be called.\nDrag off pins to build functionality.
)

(event EventInteractwithObject
  (params (PlayerReference :type BP%20Third%20Person%20Character%20Object%20Reference))
  (bind _charactermovement (Variables|/Script/Engine.Character|GetCharacterMovement PlayerReference))
  (if (Variables|Default|GetIsChosen)
    (Pawn|Components|CharacterMovement|DisableMovement _charactermovement)
    (Variables|Default|SetCharMovementRef _charactermovement)
    (Variables|Default|SetIsChosen false)
    (Rendering|SetVisibility (Variables|Default|GetNotifWidget) false false)
    (Rendering|SetVisibility (Variables|Default|GetTutTextWidget) false false)
    (bind _returnvalue (UserInterface|CreateWidget "/Game/GameJamContent/Interactables/Office/UI/BPW_TypingBox.BPW_TypingBox_C" 0 self (Variables|Default|GetMinigameType)))
    (UserInterface|Viewport|AddtoViewport _returnvalue 0)))

(fn ConstructionScript
  (|CallParentFunction))