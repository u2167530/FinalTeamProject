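; Office watering plant interactable that runs a three-attempt timing minigame for worker happiness.
; Interacting locks player movement and starts a gauge widget; further presses score hits when progress falls within the saved target range, then reposition the target randomly.
; After the last attempt it sends earned happiness to all BP_Worker actors, restores walking and waits for a reset.
; Upgrades swap the pot material and raise happiness gained per hit.
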(event Custom|Upgrade_Event
  (Rendering|Material|SetMaterial (Variables|Default|GetPlantPot) 0 (Variables|Default|GetUpgradeMaterial))
  (Variables|Default|SetHappinessGain (+ (Variables|Default|GetHappinessGain) (/ (Variables|Default|GetUpgradeAmount) 1e+01))))

(event EventBeginPlay
  (|CallParentFunction)
  (bind _asbpw_watering_gauge (Utilities|Casting|CastToBPW_WateringGauge (UserInterface|GetWidget (Variables|Default|GetWaterGaugeWidget))))
  (Variables|Default|SetAs%20BPW%20Watering%20Gauge _asbpw_watering_gauge)
  (EventDispatchers|AssignUpgrade (delegate Custom|Upgrade_Event))
  (Variables|Default|SetIsChosen true)
  (Variables|Default|SetReadyForMinigame true)
  (CallFunction|AllowInteractions))

(event Collision|EventActorBeginOverlap
  (params (OtherActor :type Actor%20Object%20Reference)))

(event EventTick
  (params (DeltaSeconds :type Float%20%28single-precision%29)))

(event EventInteractwithObject
  (params (PlayerReference :type BP%20Third%20Person%20Character%20Object%20Reference))
  (bind _as_bpw_watering_gauge (Variables|Default|GetAs%20BPW%20Watering%20Gauge))
  (bind _targetrepositions (Variables|Default|GetTargetRepositions))
  (bind _charactermovement (Variables|/Script/Engine.Character|GetCharacterMovement PlayerReference))
  (if (Variables|Default|GetReadyForMinigame)
    (Rendering|SetVisibility (Variables|Default|GetTutTextWidget) false false)
    (if (Variables|Default|GetIsInMinigame)
      (if (not (Variables|/Game/GameJamContent/Interactables/Office/UI/BPW_WateringGauge.BPW_WateringGauge_C|GetStopGaugeInput _as_bpw_watering_gauge))
        ;[1 1 1] Checks if the gauge is on the target
        (Math|Integer|IncrementInt (Variables|Default|GetAttemptCounter)
          (:%20%20
            (if (and (>= (Variables|/Game/GameJamContent/Interactables/Office/UI/BPW_WateringGauge.BPW_WateringGauge_C|GetWaterGaugeProgress _as_bpw_watering_gauge) (- (Variables|Default|GetSavedRange) 0.2)) (<= (Variables|/Game/GameJamContent/Interactables/Office/UI/BPW_WateringGauge.BPW_WateringGauge_C|GetWaterGaugeProgress _as_bpw_watering_gauge) (+ (Variables|Default|GetSavedRange) 0.2)))
              ;[1 1 1] Replace with happy/sad sound later
              (Development|PrintString "Hit")
              (Variables|Default|SetHappinessEarned (+ (Variables|Default|GetHappinessEarned) (Variables|Default|GetHappinessGain)))
              (else
                (Development|PrintString "Miss")))
            (if (>= (Variables|Default|GetAttemptCounter) 3)
              (Variables|Default|SetIsChosen false)
              (Rendering|SetVisibility (Variables|Default|GetWaterGaugeWidget) false false) ; Hides the gauge
              (Utilities|Time|PauseTimerbyHandle (Variables|/Game/GameJamContent/Interactables/Office/UI/BPW_WateringGauge.BPW_WateringGauge_C|GetWaterEvent (Variables|Default|GetAs%20BPW%20Watering%20Gauge))) ; Stops the gauge
              (Variables|Default|SetAttemptCounter 0)
              (Variables|Default|SetIsInMinigame false)
              (Variables|/Game/GameJamContent/Interactables/Office/UI/BPW_WateringGauge.BPW_WateringGauge_C|SetWaterGaugeProgress (Variables|Default|GetAs%20BPW%20Watering%20Gauge) 0.0)
              (bind _outactors (Actor|GetAllActorsOfClass "/Game/GameJamContent/Workers/Blueprint/BP_Worker.BP_Worker_C"))
              (for _array_element _outactors
                (Class|BPiWorker|ReceiveMinigameBonus(Message) _array_element (Variables|Default|GetHappinessEarned) (Variables|Default|GetMinigameType)))
              (Pawn|Components|CharacterMovement|SetMovementMode (Variables|Default|GetCharMovementRef) "MOVE_Walking" 0)
              (Variables|Default|SetReadyForMinigame false)
              (Variables|Default|SetHappinessEarned 0.0)
              (else
                (bind _output_get (Variables|Default|SetSavedInt (.OutIndex (Utilities|Array|Random _targetrepositions))))
                (bind _output_get_2 (Variables|Default|SetSavedReposition (Utilities|Array|Get(acopy) _targetrepositions _output_get)))
                (Variables|Default|SetSavedRange (Utilities|Array|Get(acopy) (Variables|Default|GetRange) _output_get))
                (Class|CanvasPanelSlot|SetPosition (Class|WidgetLayoutLibrary|SlotasCanvasSlot (Variables|/Game/GameJamContent/Interactables/Office/UI/BPW_WateringGauge.BPW_WateringGauge_C|GetGaugeTarget (Variables|Default|GetAs%20BPW%20Watering%20Gauge))) (Math|Vector2D|MakeVector2D _output_get_2 -35.0)))))))
      (else
        (Pawn|Components|CharacterMovement|DisableMovement _charactermovement)
        (Variables|Default|SetCharMovementRef _charactermovement)
        ;[1 1 1] Displays water gauge, hides "!"
        (Rendering|SetVisibility (Variables|Default|GetWaterGaugeWidget) true false)
        (Rendering|SetVisibility (Variables|Default|GetNotifWidget) false false)
        (Variables|Default|SetIsInMinigame true)
        (Default|StartTimer (Variables|Default|GetAs%20BPW%20Watering%20Gauge))))))

(event EventResetMinigame
  (Variables|Default|SetReadyForMinigame true))

(fn ConstructionScript
  (|CallParentFunction))