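; BP_Glasses is an interactable office accessory pickup for glasses that the player can carry.
; On begin play it applies its accessory mesh and sets a hardcoded attachment transform.
; Interacting with empty hands shows closed glasses on the player's Weapon mesh, copies accessory type, mesh, transform and respawn location to the player, then destroys the pickup.
; An unconnected leftover branch would put a hat mesh on a random worker.
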(event EventBeginPlay
  (Components|StaticMesh|SetStaticMesh (Variables|Default|GetStaticMesh) (Variables|Default|GetAccessoryMesh))
  (Variables|Default|SetAccessoryTransform (Math|Transform|MakeTransform "4.000000,0.000000,-130.000000" "0.000000,180.000000,-180.000000" "7.000000,7.000000,7.000000")))

(event Collision|EventActorBeginOverlap
  (params (OtherActor :type Actor%20Object%20Reference)))

(event EventTick
  (params (DeltaSeconds :type Float%20%28single-precision%29)))

(event EventInteractwithObject
  (params (PlayerReference :type BP%20Third%20Person%20Character%20Object%20Reference))
  (bind _weapon (Variables|/Game/GameJamContent/Player/Blueprint/BP_ThirdPersonCharacter.BP_ThirdPersonCharacter_C|GetWeapon PlayerReference))
  (if (not (Variables|/Game/GameJamContent/Player/Blueprint/BP_ThirdPersonCharacter.BP_ThirdPersonCharacter_C|GetisCarryingItem PlayerReference))
    (Components|StaticMesh|SetStaticMesh _weapon "/Game/GameJamContent/Workers/AccessoryModels/EmployeeProps_Glasses_Closed.EmployeeProps_Glasses_Closed")
    (Transformation|SetRelativeScale3D _weapon "0.500000,0.500000,0.500000")
    (Variables|/Game/GameJamContent/Player/Blueprint/BP_ThirdPersonCharacter.BP_ThirdPersonCharacter_C|SetAccessoryMesh PlayerReference "/Game/GameJamContent/Workers/AccessoryModels/EmployeeProps_Glasses_Closed.EmployeeProps_Glasses_Closed")
    (Variables|/Game/GameJamContent/Player/Blueprint/BP_ThirdPersonCharacter.BP_ThirdPersonCharacter_C|SetInteractionType PlayerReference "NewEnumerator2")
    (Variables|/Game/GameJamContent/Player/Blueprint/BP_ThirdPersonCharacter.BP_ThirdPersonCharacter_C|SetAccessoryTransform PlayerReference (Variables|Default|GetAccessoryTransform))
    (Variables|/Game/GameJamContent/Player/Blueprint/BP_ThirdPersonCharacter.BP_ThirdPersonCharacter_C|SetisCarryingItem PlayerReference true)
    (Variables|/Game/GameJamContent/Player/Blueprint/BP_ThirdPersonCharacter.BP_ThirdPersonCharacter_C|SetAccRespawnLoc PlayerReference (Transformation|GetWorldLocation (Variables|Default|GetDefaultSceneRoot)))
    (Actor|DestroyActor)))

(fn ConstructionScript)