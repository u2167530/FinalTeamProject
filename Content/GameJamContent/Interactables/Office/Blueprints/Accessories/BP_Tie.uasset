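; BP_Tie is an office accessory pickup that the player can carry.
; On BeginPlay it applies its accessory mesh and sets a hard-coded transform for it.
; On interaction, if IsCarryingCoffee is false, it puts the mesh on the player's Weapon component, rescales it and passes mesh, transform and interaction type to the player.
; It then sets IsCarryingCoffee, which serves as the carry flag here, and destroys itself.
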(event EventBeginPlay
  (Components|StaticMesh|SetStaticMesh (Variables|Default|GetStaticMesh) (Variables|Default|GetAccessoryMesh))
  (Variables|Default|SetAccessoryTransform (Math|Transform|MakeTransform "0, 0, 0" "0.000000,-90.000000,90.000000" "1.000000,0.250000,0.250000")))

(event Collision|EventActorBeginOverlap
  (params (OtherActor :type Actor%20Object%20Reference)))

(event EventTick
  (params (DeltaSeconds :type Float%20%28single-precision%29)))

(event EventInteractwithObject
  (params (PlayerReference :type BP%20Third%20Person%20Character%20Object%20Reference))
  (bind _staticmesh (Variables|Default|GetStaticMesh))
  (bind _weapon (Variables|/Game/GameJamContent/Player/Blueprint/BP_ThirdPersonCharacter.BP_ThirdPersonCharacter_C|GetWeapon PlayerReference))
  (bind _staticmesh_2 (Variables|/Script/Engine.StaticMeshComponent|GetStaticMesh _staticmesh))
  (if (not (Variables|/Game/GameJamContent/Player/Blueprint/BP_ThirdPersonCharacter.BP_ThirdPersonCharacter_C|GetisCarryingCoffee PlayerReference))
    (Components|StaticMesh|SetStaticMesh _weapon _staticmesh_2)
    (Transformation|SetRelativeScale3D _weapon "1.000000,0.250000,0.250000")
    (Variables|/Game/GameJamContent/Player/Blueprint/BP_ThirdPersonCharacter.BP_ThirdPersonCharacter_C|SetAccessoryMesh PlayerReference _staticmesh_2)
    (Variables|/Game/GameJamContent/Player/Blueprint/BP_ThirdPersonCharacter.BP_ThirdPersonCharacter_C|SetInteractionType PlayerReference "NewEnumerator4")
    (Variables|/Game/GameJamContent/Player/Blueprint/BP_ThirdPersonCharacter.BP_ThirdPersonCharacter_C|SetAccessoryTransform PlayerReference (Variables|Default|GetAccessoryTransform))
    (Variables|/Game/GameJamContent/Player/Blueprint/BP_ThirdPersonCharacter.BP_ThirdPersonCharacter_C|SetisCarryingCoffee PlayerReference true)
    (Actor|DestroyActor)))

(fn ConstructionScript)