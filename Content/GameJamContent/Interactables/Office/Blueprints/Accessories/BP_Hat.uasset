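; BP_Hat is an interactable hat accessory in the office that the player can pick up.
; BeginPlay applies its mesh and sets a scaled-up accessory transform.
; On interaction, if IsCarryingCoffee is false, it shows the hat on the player's Weapon mesh, passes over mesh, type, transform and respawn location, sets that flag, then destroys itself.
; Unconnected leftover logic would put the hat on a random BP_Worker's head.
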(event EventBeginPlay
  (Components|StaticMesh|SetStaticMesh (Variables|Default|GetStaticMesh) (Variables|Default|GetAccessoryMesh))
  (Variables|Default|SetAccessoryTransform (Math|Transform|MakeTransform "0, 0, 0" "0, 0, 0" "5.000000,5.000000,5.000000")))

(event Collision|EventActorBeginOverlap
  (params (OtherActor :type Actor%20Object%20Reference)))

(event EventTick
  (params (DeltaSeconds :type Float%20%28single-precision%29)))

(event EventInteractwithObject
  (params (PlayerReference :type BP%20Third%20Person%20Character%20Object%20Reference))
  (bind _staticmesh (Variables|Default|GetStaticMesh))
  (bind _weapon (Variables|/Game/GameJamContent/Player/Blueprint/BP_ThirdPersonCharacter.BP_ThirdPersonCharacter_C|GetWeapon PlayerReference))
  (bind _staticmesh_2 (Variables|/Script/Engine.StaticMeshComponent|GetStaticMesh _staticmesh))
  (if (not (Variables|/Game/GameJamContent/Player/Blueprint/BP_ThirdPersonCharacter.BP_ThirdPersonCharacter_C|GetisCarryingCoffee PlayerReference))
    (Components|StaticMesh|SetStaticMesh _weapon _staticmesh_2)
    (Transformation|SetRelativeScale3D _weapon "0.500000,0.500000,0.500000")
    (Variables|/Game/GameJamContent/Player/Blueprint/BP_ThirdPersonCharacter.BP_ThirdPersonCharacter_C|SetAccessoryMesh PlayerReference _staticmesh_2)
    (Variables|/Game/GameJamContent/Player/Blueprint/BP_ThirdPersonCharacter.BP_ThirdPersonCharacter_C|SetInteractionType PlayerReference "NewEnumerator1")
    (Variables|/Game/GameJamContent/Player/Blueprint/BP_ThirdPersonCharacter.BP_ThirdPersonCharacter_C|SetAccessoryTransform PlayerReference (Variables|Default|GetAccessoryTransform))
    (Variables|/Game/GameJamContent/Player/Blueprint/BP_ThirdPersonCharacter.BP_ThirdPersonCharacter_C|SetisCarryingCoffee PlayerReference true)
    (Variables|/Game/GameJamContent/Player/Blueprint/BP_ThirdPersonCharacter.BP_ThirdPersonCharacter_C|SetAccRespawnLoc PlayerReference (Transformation|GetWorldLocation (Variables|Default|GetDefaultSceneRoot)))
    (Actor|DestroyActor)))

(fn ConstructionScript)