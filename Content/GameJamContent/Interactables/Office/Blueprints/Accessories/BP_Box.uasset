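; BP_Box is an office accessory box that the player picks up by interacting with it.
; If the player is not already carrying an item, it copies its mesh to the player's ItemHand at half scale and sets the carrying flag, accessory mesh and interaction type.
; It also saves its world location to the player's AccRespawnLoc, then destroys itself.
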(event EventBeginPlay)

(event Collision|EventActorBeginOverlap
  (params (OtherActor :type Actor%20Object%20Reference)))

(event EventTick
  (params (DeltaSeconds :type Float%20%28single-precision%29)))

(event EventInteractwithObject
  (params (PlayerReference :type BP%20Third%20Person%20Character%20Object%20Reference))
  (bind _staticmesh (Variables|Default|GetStaticMesh))
  (bind _itemhand (Variables|/Game/GameJamContent/Player/Blueprint/BP_ThirdPersonCharacter.BP_ThirdPersonCharacter_C|GetItemHand PlayerReference))
  (bind _staticmesh_2 (Variables|/Script/Engine.StaticMeshComponent|GetStaticMesh _staticmesh))
  (if (not (Variables|/Game/GameJamContent/Player/Blueprint/BP_ThirdPersonCharacter.BP_ThirdPersonCharacter_C|GetisCarryingItem PlayerReference))
    (Components|StaticMesh|SetStaticMesh _itemhand _staticmesh_2)
    (Transformation|SetRelativeScale3D _itemhand "0.500000,0.500000,0.500000")
    (Variables|/Game/GameJamContent/Player/Blueprint/BP_ThirdPersonCharacter.BP_ThirdPersonCharacter_C|SetAccessoryMesh PlayerReference _staticmesh_2)
    (Variables|/Game/GameJamContent/Player/Blueprint/BP_ThirdPersonCharacter.BP_ThirdPersonCharacter_C|SetInteractionType PlayerReference "NewEnumerator5")
    (Variables|/Game/GameJamContent/Player/Blueprint/BP_ThirdPersonCharacter.BP_ThirdPersonCharacter_C|SetisCarryingItem PlayerReference true)
    (Variables|/Game/GameJamContent/Player/Blueprint/BP_ThirdPersonCharacter.BP_ThirdPersonCharacter_C|SetAccRespawnLoc PlayerReference (Transformation|GetWorldLocation (Variables|Default|GetDefaultSceneRoot)))
    (Actor|DestroyActor)))

(fn ConstructionScript)