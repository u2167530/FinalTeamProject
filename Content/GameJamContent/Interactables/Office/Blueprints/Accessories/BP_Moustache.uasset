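; BP_Moustache is an interactable moustache accessory pickup that the player can carry.
; BeginPlay applies the accessory mesh and sets a fixed attach transform.
; On interact, an empty-handed player's Weapon mesh shows the moustache with a placeholder material, and the player receives its mesh, type, transform and respawn location before the pickup destroys itself.
; Unconnected leftover nodes would put hat meshes on a random BP_Worker.
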(event EventBeginPlay
  (Components|StaticMesh|SetStaticMesh (Variables|Default|GetStaticMesh) (Variables|Default|GetAccessoryMesh))
  (Variables|Default|SetAccessoryTransform (Math|Transform|MakeTransform "15.000000,0.000000,-170.000000" "0.000000,-180.000000,0.000000" "7.000000,7.000000,7.000000")))

(event Collision|EventActorBeginOverlap
  (params (OtherActor :type Actor%20Object%20Reference)))

(event EventTick
  (params (DeltaSeconds :type Float%20%28single-precision%29)))

(event EventInteractwithObject
  (params (PlayerReference :type BP%20Third%20Person%20Character%20Object%20Reference))
  (bind _weapon (Variables|/Game/GameJamContent/Player/Blueprint/BP_ThirdPersonCharacter.BP_ThirdPersonCharacter_C|GetWeapon PlayerReference))
  (if (not (Variables|/Game/GameJamContent/Player/Blueprint/BP_ThirdPersonCharacter.BP_ThirdPersonCharacter_C|GetisCarryingItem PlayerReference))
    ;[1 1 1] Placeholder until the textures are ready
    (Rendering|Material|SetMaterial _weapon 0 "/Game/GameJamContent/Workers/AccessoryModels/Moustache_M.Moustache_M")
    (Components|StaticMesh|SetStaticMesh _weapon (Variables|/Script/Engine.StaticMeshComponent|GetStaticMesh (Variables|Default|GetStaticMesh)))
    (Transformation|SetRelativeScale3D _weapon "1.000000,1.000000,1.000000")
    (Variables|/Game/GameJamContent/Player/Blueprint/BP_ThirdPersonCharacter.BP_ThirdPersonCharacter_C|SetAccessoryMesh PlayerReference (Variables|/Script/Engine.StaticMeshComponent|GetStaticMesh (Variables|Default|GetStaticMesh)))
    (Variables|/Game/GameJamContent/Player/Blueprint/BP_ThirdPersonCharacter.BP_ThirdPersonCharacter_C|SetInteractionType PlayerReference "NewEnumerator3")
    (Variables|/Game/GameJamContent/Player/Blueprint/BP_ThirdPersonCharacter.BP_ThirdPersonCharacter_C|SetAccessoryTransform PlayerReference (Variables|Default|GetAccessoryTransform))
    (Variables|/Game/GameJamContent/Player/Blueprint/BP_ThirdPersonCharacter.BP_ThirdPersonCharacter_C|SetisCarryingItem PlayerReference true)
    (Variables|/Game/GameJamContent/Player/Blueprint/BP_ThirdPersonCharacter.BP_ThirdPersonCharacter_C|SetAccRespawnLoc PlayerReference (Transformation|GetWorldLocation (Variables|Default|GetDefaultSceneRoot)))
    (Actor|DestroyActor)))

(fn ConstructionScript)