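; Interactable office coffee machine that brews a coffee for the player while they hold interact.
; A box overlap gates brewing and shows the pop-up, and leaving the box resets any progress.
; InteractwithObject starts a looping timer that fills a widget progress bar, while HoldInteract cancels and resets it.
; A full gauge flags the player as carrying coffee and calls NeedsCoffee on every BP_Worker.
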(event OnComponentBeginOverlap(Box)
  (params (OverlappedComponent :type Primitive%20Component%20Object%20Reference) (OtherActor :type Actor%20Object%20Reference) (OtherComp :type Primitive%20Component%20Object%20Reference) (OtherBodyIndex :type Integer) (bFromSweep :type Boolean) (SweepResult :type Hit%20Result%20Structure%20%28by%20ref%29))
  (if (Utilities|DoesObjectImplementInterface OtherActor "/Game/GameJamContent/Player/BPi_Player.BPi_Player_C")
    (Utilities|IsValid (Variables|Default|GetPlayerReference)
      (:Is%20Valid
        (if (Variables|/Game/GameJamContent/Player/Blueprint/BP_ThirdPersonCharacter.BP_ThirdPersonCharacter_C|GetisCarryingCoffee (Variables|Default|GetPlayerReference))
          (Rendering|SetVisibility (Variables|Default|GetInteractablePopUp) false false)
          (Variables|Default|SetCanMakeCoffee false)
          (else
            (Rendering|SetVisibility (Variables|Default|GetInteractablePopUp) true false)
            (Variables|Default|SetCanMakeCoffee true))))
      (:Is%20Not%20Valid
        (Rendering|SetVisibility (Variables|Default|GetInteractablePopUp) true false)
        (Variables|Default|SetCanMakeCoffee true) ; Enables player to interact with the coffee machine
      ))))

(event OnComponentEndOverlap(Box)
  (params (OverlappedComponent :type Primitive%20Component%20Object%20Reference) (OtherActor :type Actor%20Object%20Reference) (OtherComp :type Primitive%20Component%20Object%20Reference) (OtherBodyIndex :type Integer))
  (if (Utilities|DoesObjectImplementInterface OtherActor "/Game/GameJamContent/Player/BPi_Player.BPi_Player_C")
    (Rendering|SetVisibility (Variables|Default|GetInteractablePopUp) false false)
    (Variables|Default|SetCanMakeCoffee false) ; Disables interacting with the coffee machine
    (Rendering|SetVisibility (Variables|Default|GetCoffeeGauge) false false)
    (Variables|Default|SetCoffeeProgress 0.0)
    (Progress|SetPercent (Variables|/Game/GameJamContent/Interactables/Office/UI/BPW_CoffeeMachineGauge.BPW_CoffeeMachineGauge_C|GetCoffeeProgressBar (Variables|Default|GetCoffeeUIRef)) 0.0)
    (Class|KismetSystemLibrary|PauseTimer 0 "IncreaseCoffeeGauge")))

(event EventBeginPlay
  ;[1 1 1] Sets up relevant references
  (bind _asbpw_coffee_machine_gauge (Utilities|Casting|CastToBPW_CoffeeMachineGauge (UserInterface|GetUserWidgetObject (Variables|Default|GetCoffeeGauge))))
  (Variables|Default|SetCoffeeUIRef _asbpw_coffee_machine_gauge))

(event EventInteractwithObject
  (params (PlayerReference :type BP%20Third%20Person%20Character%20Object%20Reference))
  ;[1 1 1] Displays the coffee gauge and increases it every 0.2 seconds whilst the player is holding the interact key
  (bind _output_get (Variables|Default|SetPlayerReference PlayerReference))
  (if (and (Variables|Default|GetCanMakeCoffee) (Variables|/Game/GameJamContent/Player/Blueprint/BP_ThirdPersonCharacter.BP_ThirdPersonCharacter_C|GetCanMakeCoffee _output_get))
    (Rendering|SetVisibility (Variables|Default|GetInteractablePopUp) false false)
    (Rendering|SetVisibility (Variables|Default|GetCoffeeGauge) true false)
    (Utilities|Time|SetTimerbyFunctionName 0 "IncreaseCoffeeGauge" 0.2 true)))

(event EventHoldInteract
  (if (and (Variables|/Game/GameJamContent/Player/Blueprint/BP_ThirdPersonCharacter.BP_ThirdPersonCharacter_C|GetCanMakeCoffee (Variables|Default|GetPlayerReference)) (Variables|Default|GetCanMakeCoffee))
    ;[1 1 1] Hides coffee gauge, displays interactable pop-up and resets values related to the coffee gauge
    (Rendering|SetVisibility (Variables|Default|GetCoffeeGauge) false false)
    (Rendering|SetVisibility (Variables|Default|GetInteractablePopUp) true false)
    (Variables|Default|SetCoffeeProgress 0.0)
    (Progress|SetPercent (Variables|/Game/GameJamContent/Interactables/Office/UI/BPW_CoffeeMachineGauge.BPW_CoffeeMachineGauge_C|GetCoffeeProgressBar (Variables|Default|GetCoffeeUIRef)) 0.0)
    (Class|KismetSystemLibrary|PauseTimer 0 "IncreaseCoffeeGauge")))

(fn ConstructionScript)

(fn IncreaseCoffeeGauge
  (bind _playerreference (Variables|Default|GetPlayerReference))
  ;[1 1 1] Adds 5% to the coffee gauge
  (bind _output_get (Variables|Default|SetCoffeeProgress (+ (Variables|Default|GetCoffeeProgress) 5.0)))
  (Progress|SetPercent (Variables|/Game/GameJamContent/Interactables/Office/UI/BPW_CoffeeMachineGauge.BPW_CoffeeMachineGauge_C|GetCoffeeProgressBar (Variables|Default|GetCoffeeUIRef)) (/ _output_get 1e+02))
  (if (>= (Variables|Default|GetCoffeeProgress) 1e+02) ; is the coffee gauge full
    ;[1 1 1] This is where you get the coffee
    (Variables|/Game/GameJamContent/Player/Blueprint/BP_ThirdPersonCharacter.BP_ThirdPersonCharacter_C|SetisCarryingCoffee _playerreference true)
    (Variables|/Game/GameJamContent/Player/Blueprint/BP_ThirdPersonCharacter.BP_ThirdPersonCharacter_C|SetCanMakeCoffee _playerreference false)
    (Development|PrintString "Got Coffee!!!")
    ;[1 1 1] Hides coffee gauge, reduces values related to it to 0 and pauses the timer
    (Rendering|SetVisibility (Variables|Default|GetCoffeeGauge) false false)
    (Variables|Default|SetCoffeeProgress 0.0)
    (Progress|SetPercent (Variables|/Game/GameJamContent/Interactables/Office/UI/BPW_CoffeeMachineGauge.BPW_CoffeeMachineGauge_C|GetCoffeeProgressBar (Variables|Default|GetCoffeeUIRef)) 0.0)
    (Class|KismetSystemLibrary|PauseTimer 0 "IncreaseCoffeeGauge")
    (bind _outactors (Actor|GetAllActorsOfClass "/Game/GameJamContent/Workers/Blueprint/BP_Worker.BP_Worker_C"))
    (for _array_element _outactors
      (Default|NeedsCoffee _array_element))))