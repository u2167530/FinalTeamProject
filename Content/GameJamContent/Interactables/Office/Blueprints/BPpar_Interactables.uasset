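; Parent Blueprint for office interactables that marks itself ready for a minigame while a player is inside its interaction box.
; Overlaps with BPi_Player actors toggle ReadyForMinigame and a tutorial widget, with one minigame type also requiring the object to be chosen and enabled.
; AllowInteractions and StopInteractions toggle that state and a notification widget, with Allow also showing the tutorial if the player already overlaps.
; SetasUsable is an unused leftover from minigame randomisation.
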(event OnComponentBeginOverlap(InteractableBox)
  (params (OverlappedComponent :type Primitive%20Component%20Object%20Reference) (OtherActor :type Actor%20Object%20Reference) (OtherComp :type Primitive%20Component%20Object%20Reference) (OtherBodyIndex :type Integer) (bFromSweep :type Boolean) (SweepResult :type Hit%20Result%20Structure%20%28by%20ref%29))
  (if (Utilities|DoesObjectImplementInterface OtherActor "/Game/GameJamContent/Player/BPi_Player.BPi_Player_C")
    (if (Utilities|Enum|Equal(Enum) (Variables|Default|GetMinigameType) "NewEnumerator2")
      (if (and (not (Variables|Default|GetDisableCollision)) (Variables|Default|GetIsChosen))
        (Variables|Default|SetReadyForMinigame true :!label _label)
        (Rendering|SetVisibility (Variables|Default|GetTutTextWidget) true false))
      (else
        (goto _label)))))

(event OnComponentEndOverlap(InteractableBox)
  (params (OverlappedComponent :type Primitive%20Component%20Object%20Reference) (OtherActor :type Actor%20Object%20Reference) (OtherComp :type Primitive%20Component%20Object%20Reference) (OtherBodyIndex :type Integer))
  (if (Utilities|DoesObjectImplementInterface OtherActor "/Game/GameJamContent/Player/BPi_Player.BPi_Player_C")
    (if (Utilities|Enum|Equal(Enum) (Variables|Default|GetMinigameType) "NewEnumerator2")
      (if (and (not (Variables|Default|GetDisableCollision)) (Variables|Default|GetIsChosen))
        (Variables|Default|SetReadyForMinigame false :!label _label)
        (Rendering|SetVisibility (Variables|Default|GetTutTextWidget) false false))
      (else
        (goto _label)))))

(event Custom|StopInteractions
  (Rendering|SetVisibility (Variables|Default|GetNotifWidget) false false)
  (Variables|Default|SetIsChosen false)
  (Variables|Default|SetDisableCollision true)
  (Rendering|SetVisibility (Variables|Default|GetTutTextWidget) false false))

(event EventBeginPlay
  (bind _asbpw_interact_notif (Utilities|Casting|CastToBPW_InteractNotif (UserInterface|GetWidget (Variables|Default|GetNotifWidget))))
  (Variables|Default|SetAs%20BPW%20Interact%20Notif _asbpw_interact_notif))

(event EventSetasUsable
  (params (Enable? :type Boolean))
  ;[1 1 1] Unused (formerly used for randomising minigames)
)

(event EventAllowInteractions
  (Rendering|SetVisibility (Variables|Default|GetNotifWidget) true false)
  (Variables|Default|SetIsChosen true)
  (Variables|Default|SetDisableCollision false)
  (if (Collision|IsOverlappingActor (Variables|Default|GetInteractableBox) (Game|Player|GetPlayerPawn 0) :!class /Script/Engine.PrimitiveComponent)
    (Rendering|SetVisibility (Variables|Default|GetTutTextWidget) true false)))

(fn ConstructionScript)