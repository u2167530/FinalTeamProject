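; BP_WateringGauge is an office interactable that runs a timing minigame on a watering gauge.
; When ready, the first interaction hides the notification widget, shows the gauge and starts the timer on its BPW_WateringGauge widget.
; Each further interaction checks whether the widget's progress sits in the middle target band, only printing Hit or Miss.
; After three attempts it hides the gauge and pauses the timer; the attempt counter is never reset.
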(event EventBeginPlay
  (|CallParentFunction)
  (bind _asbpw_watering_gauge (Utilities|Casting|CastToBPW_WateringGauge (UserInterface|GetWidget (Variables|Default|GetWaterGaugeWidget))))
  (Variables|Default|SetAs%20BPW%20Watering%20Gauge _asbpw_watering_gauge))

(event Collision|EventActorBeginOverlap
  (params (OtherActor :type Actor%20Object%20Reference)))

(event EventTick
  (params (DeltaSeconds :type Float%20%28single-precision%29)))

(event EventInteractwithObject
  (bind _as_bpw_watering_gauge (Variables|Default|GetAs%20BPW%20Watering%20Gauge))
  (bind _watergaugeprogress (Variables|/Game/GameJamContent/Interactables/Office/UI/BPW_WateringGauge.BPW_WateringGauge_C|GetWaterGaugeProgress _as_bpw_watering_gauge))
  (if (Variables|Default|GetReadyForMinigame)
    (if (Variables|Default|GetIsInMinigame)
      ;[1 1 1] Checks if the gauge is on the target
      (Math|Integer|IncrementInt (Variables|Default|GetAttemptCounter)
        (:%20%20
          (if (and (>= _watergaugeprogress 0.4) (<= _watergaugeprogress 0.6))
            (Development|PrintString "Hit")
            (else
              (Development|PrintString "Miss")))
          (if (>= (Variables|Default|GetAttemptCounter) 3)
            (Variables|Default|SetIsInMinigame false)
            (Rendering|SetVisibility (Variables|Default|GetWaterGaugeWidget) false false)
            (Utilities|Time|PauseTimerbyHandle (Variables|/Game/GameJamContent/Interactables/Office/UI/BPW_WateringGauge.BPW_WateringGauge_C|GetWaterEvent (Variables|Default|GetAs%20BPW%20Watering%20Gauge))))))
      (else
        ;[1 1 1] Displays water gauge, hides "!"
        (Rendering|SetVisibility (Variables|Default|GetWaterGaugeWidget) true false)
        (Rendering|SetVisibility (Variables|Default|GetNotifWidget) false false)
        (Variables|Default|SetIsInMinigame true)
        (Default|StartTimer (Variables|Default|GetAs%20BPW%20Watering%20Gauge))))))

(fn ConstructionScript
  (|CallParentFunction))