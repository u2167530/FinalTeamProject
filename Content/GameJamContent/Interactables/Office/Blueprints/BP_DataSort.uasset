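; BP_DataSort is an office interactable that opens the data sort widget for the player.
; On BeginPlay it caches a reference to the BPW_DataSort instance hosted in its DataSortWidget component.
; InteractwithObject creates a separate BPW_DataSort and adds it to the viewport when IsChosen is true, leaving the cached component widget unused.
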(event EventBeginPlay
  (|CallParentFunction)
  (bind _asbpw_data_sort (Utilities|Casting|CastToBPW_DataSort (UserInterface|GetWidget (Variables|Default|GetDataSortWidget))))
  (Variables|Default|SetDataSortWIdgetRef _asbpw_data_sort))

(event Collision|EventActorBeginOverlap
  (params (OtherActor :type Actor%20Object%20Reference))
  (|CallParentFunction OtherActor) ; This node is disabled and will not be called.\nDrag off pins to build functionality.
)

(event EventTick
  (params (DeltaSeconds :type Float%20%28single-precision%29))
  (|CallParentFunction DeltaSeconds) ; This node is disabled and will not be called.\nDrag off pins to build functionality.
)

(event EventInteractwithObject
  (params (PlayerReference :type BP%20Third%20Person%20Character%20Object%20Reference))
  (if (Variables|Default|GetIsChosen)
    (bind _returnvalue (UserInterface|CreateWidget "/Game/GameJamContent/Interactables/Office/UI/BPW_DataSort.BPW_DataSort_C"))
    (UserInterface|Viewport|AddtoViewport _returnvalue 0)))

(fn ConstructionScript
  (|CallParentFunction))