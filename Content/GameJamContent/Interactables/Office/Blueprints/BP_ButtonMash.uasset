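; Office interactable that runs a button-mash minigame when it is the chosen task.
; The first interaction locks player movement and opens a BPW_ButtonMash gauge; each further interaction fills it.
; A full gauge notifies completion, sends a happiness bonus to all BP_Worker actors and restores walking, while closing or stopping also removes the gauge.
; A bound upgrade event enables reduced breakdown using the upgrade amount as its time.
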(event Custom|Upgrade_Event
  (Variables|Default|SetBreakdownReduced true)
  (Variables|Default|SetBreakdownReducedTime (Variables|Default|GetUpgradeAmount)))

(event Custom|CloseMinigame
  (Widget|RemovefromParent (Variables|Default|GetBMGaugeRef))
  (Variables|Default|SetIsInMinigame false)
  (Rendering|SetVisibility (Variables|Default|GetTutTextWidget) true false)
  (Pawn|Components|CharacterMovement|SetMovementMode (Variables|Default|GetCharMovementRef) "MOVE_Walking" 0)
  (Input|SetInputModeGameOnly (Game|GetPlayerController 0) false))

(event EventBeginPlay
  (|CallParentFunction)
  (EventDispatchers|BindEventtoUpgrade (delegate Custom|Upgrade_Event)))

(event Collision|EventActorBeginOverlap
  (params (OtherActor :type Actor%20Object%20Reference))
  (|CallParentFunction OtherActor) ; This node is disabled and will not be called.\nDrag off pins to build functionality.
)

(event EventTick
  (params (DeltaSeconds :type Float%20%28single-precision%29))
  (|CallParentFunction DeltaSeconds) ; This node is disabled and will not be called.\nDrag off pins to build functionality.
)

(event EventInteractwithObject
  (params (PlayerReference :type BP%20Third%20Person%20Character%20Object%20Reference))
  (bind _charactermovement (Variables|/Script/Engine.Character|GetCharacterMovement PlayerReference))
  (if (Variables|Default|GetIsChosen)
    (Variables|Default|SetFinished false)
    (if (Variables|Default|GetIsInMinigame) ; Checks if this is the first time this is being interacted with
      ;[1 1 1] Increments how much the player has mashed and checks to see if they've mashed enough
      (Variables|/Game/GameJamContent/Interactables/Office/UI/BPW_ButtonMash.BPW_ButtonMash_C|SetBMGaugeValue (Variables|Default|GetBMGaugeRef) (+ (Variables|/Game/GameJamContent/Interactables/Office/UI/BPW_ButtonMash.BPW_ButtonMash_C|GetBMGaugeValue (Variables|Default|GetBMGaugeRef)) 0.0714))
      (if (>= (Variables|/Game/GameJamContent/Interactables/Office/UI/BPW_ButtonMash.BPW_ButtonMash_C|GetBMGaugeValue (Variables|Default|GetBMGaugeRef)) 0.98)
        (Utilities|FlowControl|Delay 0.1)
        ;[1 1 1] Hides the gauge and prevents player from repeating the minigame
        (Widget|RemovefromParent (Variables|Default|GetBMGaugeRef))
        (Rendering|SetVisibility (Variables|Default|GetNotifWidget) false false)
        (Variables|Default|SetIsInMinigame false)
        (Variables|Default|SetFinished true)
        (Variables|Default|SetIsChosen false)
        (Default|CallNotifyDone self)
        (Variables|/Game/GameJamContent/Interactables/Office/UI/BPW_ButtonMash.BPW_ButtonMash_C|SetBMGaugeValue (Variables|Default|GetBMGaugeRef) 0.0)
        (Variables|Default|SetSecondsLeft 5)
        (Rendering|Components|TextRender|SetText (Variables|/Game/GameJamContent/Interactables/Office/UI/BPW_ButtonMash.BPW_ButtonMash_C|GetTimerText (Variables|Default|GetBMGaugeRef)) "5")
        (bind _outactors (Actor|GetAllActorsOfClass "/Game/GameJamContent/Workers/Blueprint/BP_Worker.BP_Worker_C"))
        (for _array_element _outactors
          (Class|BPiWorker|ReceiveMinigameBonus(Message) _array_element 0.1 (Variables|Default|GetMinigameType)))
        (Pawn|Components|CharacterMovement|SetMovementMode (Variables|Default|GetCharMovementRef) "MOVE_Walking" 0))
      (elif (not (Variables|Default|GetFinished)) ; Checks if the player has already done this minigame
        (Pawn|Components|CharacterMovement|DisableMovement _charactermovement)
        (Variables|Default|SetCharMovementRef _charactermovement)
        (Variables|Default|SetIsInMinigame true)
        (bind _returnvalue (UserInterface|CreateWidget "/Game/GameJamContent/Interactables/Office/UI/BPW_ButtonMash.BPW_ButtonMash_C"))
        (UserInterface|Viewport|AddtoViewport _returnvalue 0)
        ;[1 1 1] Starts minigame
        (bind _output_get (Variables|Default|SetBMGaugeRef _returnvalue))
        (Variables|/Game/GameJamContent/Interactables/Office/UI/BPW_ButtonMash.BPW_ButtonMash_C|SetBPRef _output_get self)
        (Rendering|SetVisibility (Variables|Default|GetTutTextWidget) false false)
        (Input|SetInputModeGameandUI (Game|GetPlayerController 0) 0 "DoNotLock" true false)))))

(event EventStopInteractions
  (bind _charmovementref (Variables|Default|GetCharMovementRef))
  (bind _bmgaugeref (Variables|Default|GetBMGaugeRef))
  (|CallParentFunction)
  (Rendering|SetVisibility (Variables|Default|GetNotifWidget) false false)
  (Utilities|IsValid _charmovementref
    (:Is%20Valid
      (Pawn|Components|CharacterMovement|SetMovementMode _charmovementref "MOVE_Walking" 0))
    (:Is%20Not%20Valid
      _))
  (Utilities|IsValid _bmgaugeref
    (:Is%20Valid
      (Widget|RemovefromParent _bmgaugeref))))

(fn ConstructionScript
  (|CallParentFunction))