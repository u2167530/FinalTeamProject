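; Office coffee machine interactable, a child Blueprint that runs a hold-to-fill minigame to give the player coffee.
; When ready, InteractwithObject shows the gauge widget and starts a looping timer that steadily fills its progress bar.
; A full gauge sets IsCarryingCoffee on the player pawn, cast to a specific test character copy, then resets.
; HoldInteract hides and resets the gauge and pauses the timer.
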(event Custom|IncreaseCoffeeGauge
  ;[1 1 1] Increases progress bar
  (bind _output_get (Variables|Default|SetCoffeeProgress (+ (Variables|Default|GetCoffeeProgress) 5.0)))
  (Progress|SetPercent (Variables|/Game/GameJamContent/Interactables/Office/UI/BPW_CoffeeMachineGauge.BPW_CoffeeMachineGauge_C|GetCoffeeProgressBar (Variables|Default|GetCoffeeGaugeRef)) (/ _output_get 1e+02))
  (if (>= (Variables|Default|GetCoffeeProgress) 1e+02) ; Is the coffee gauge full?
    ;[1 1 1] This should cast to the base character eventually
    (bind _asbp_third_person_character_jack_copy_for_ryan (Utilities|Casting|CastToBP_ThirdPersonCHaracterJack_CopyForRyan (Game|Player|GetPlayerPawn 0)))
    (bind _output_get_2 (Variables|Default|SetPlayerRyanRef _asbp_third_person_character_jack_copy_for_ryan))
    ;[1 1 1] This is where you get the coffee
    (Variables|/Game/GameJamContent/Player/Blueprint/BP_ThirdPersonCHaracterJack_CopyForRyan.BP_ThirdPersonCHaracterJack_CopyForRyan_C|SetIsCarryingCoffee _output_get_2 true)
    (Development|PrintString "Got Coffee!!!")
    (Rendering|SetVisibility (Variables|Default|GetCoffeeWidget) false false)
    (Variables|Default|SetCoffeeProgress 0.0)
    (Progress|SetPercent (Variables|/Game/GameJamContent/Interactables/Office/UI/BPW_CoffeeMachineGauge.BPW_CoffeeMachineGauge_C|GetCoffeeProgressBar (Variables|Default|GetCoffeeGaugeRef)) 0.0)
    (Utilities|Time|PauseTimerbyHandle (Variables|Default|GetCoffeeTimerRef))))

(event EventBeginPlay
  ;[1 1 1] Sets up relevant references
  (|CallParentFunction)
  (bind _asbpw_coffee_machine_gauge (Utilities|Casting|CastToBPW_CoffeeMachineGauge (UserInterface|GetUserWidgetObject (Variables|Default|GetCoffeeWidget))))
  (Variables|Default|SetCoffeeGaugeRef _asbpw_coffee_machine_gauge))

(event Collision|EventActorBeginOverlap
  (params (OtherActor :type Actor%20Object%20Reference))
  (|CallParentFunction OtherActor) ; This node is disabled and will not be called.\nDrag off pins to build functionality.
)

(event EventTick
  (params (DeltaSeconds :type Float%20%28single-precision%29))
  (|CallParentFunction DeltaSeconds) ; This node is disabled and will not be called.\nDrag off pins to build functionality.
)

(event EventInteractwithObject
  (if (Variables|Default|GetReadyForMinigame)
    ;[1 1 1] Displays the coffee gauge and increases it every 0.2 seconds whilst the player is holding the interact key
    (Rendering|SetVisibility (Variables|Default|GetNotifWidget) false false)
    (Rendering|SetVisibility (Variables|Default|GetCoffeeWidget) true false)
    (bind _returnvalue (Utilities|Time|SetTimerbyEvent (delegate Custom|IncreaseCoffeeGauge) 0.2 true))
    (Variables|Default|SetCoffeeTimerRef _returnvalue)))

(event EventHoldInteract
  (if (Variables|Default|GetReadyForMinigame)
    ;[1 1 1] Hides coffee gauge, displays interactable pop-up and resets values related to the coffee gauge
    (Rendering|SetVisibility (Variables|Default|GetCoffeeWidget) false false)
    (Variables|Default|SetCoffeeProgress 0.0)
    (Progress|SetPercent (Variables|/Game/GameJamContent/Interactables/Office/UI/BPW_CoffeeMachineGauge.BPW_CoffeeMachineGauge_C|GetCoffeeProgressBar (Variables|Default|GetCoffeeGaugeRef)) 0.0)
    (Utilities|Time|PauseTimerbyHandle (Variables|Default|GetCoffeeTimerRef))))

(fn ConstructionScript
  (|CallParentFunction))