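; Office actor that randomly picks which interactables can be used as minigames when play begins.
; On BeginPlay it gathers all BPi_Interactable actors and drops computers by display-name match, removing them from the array mid-iteration.
; It then loops, sending AllowInteractions to a random pick and removing it to avoid repeats, until MinigameAmount reaches MinigameCap.
; Each chosen actor's name is printed for debugging.
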(event EventBeginPlay
  (bind _minigameamount (Variables|Default|GetMinigameAmount))
  (bind _outactors (Actor|GetAllActorswithInterface "/Game/GameJamContent/Interactables/Interfaces/BPi_Interactable.BPi_Interactable_C"))
  (bind _output_get (Variables|Default|SetInteractableArray _outactors))
  (for _array_element _output_get
    (if (Utilities|String|Contains (Utilities|GetDisplayName _array_element) "bp_computer")
      (Utilities|Array|RemoveItem (Variables|Default|GetInteractableArray) _array_element)))
  (Variables|Default|SetMinigameToAllow (.OutItem (Utilities|Array|Random (Variables|Default|GetInteractableArray))))
  (Class|BPiInteractable|AllowInteractions(Message) (Variables|Default|GetMinigameToAllow) :!label _label)
  (Development|PrintString (Utilities|GetDisplayName (Variables|Default|GetMinigameToAllow)))
  (Utilities|Array|RemoveItem (Variables|Default|GetInteractableArray) (Variables|Default|GetMinigameToAllow))
  (Math|Integer|IncrementInt _minigameamount
    (:%20%20
      (if (not (>= _minigameamount (Variables|Default|GetMinigameCap)))
        (Variables|Default|SetMinigameToAllow (.OutItem (Utilities|Array|Random (Variables|Default|GetInteractableArray))))
        (goto _label)))))

(event Collision|EventActorBeginOverlap
  (params (OtherActor :type Actor%20Object%20Reference)))

(event EventTick
  (params (DeltaSeconds :type Float%20%28single-precision%29)))

(fn ConstructionScript)