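; Office upgrade manager that applies purchased upgrades from the game instance when play begins.
; Minigame upgrades pass material and value to their MinigameList entry and start it; Desk and PC upgrades update every worker desk and raise a worker stat.
; UpgradeAppliances triggers upgrade calls or effects for a given list of appliance types.
; An unconnected mesh material-swap loop remains, and construction creates a dynamic material instance.
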(event Custom|UpgradeAppliances
  (params (Appliances :type Array%20of%20E_OfficeUpgrades%20Enums :default "NewEnumerator0"))
  (bind _workerdeskrefs (Variables|Default|GetWorkerDeskRefs))
  (if (not (Utilities|Array|IsEmpty Appliances))
    (for _array_element Appliances
      (switch Utilities|FlowControl|Switch|SwitchonE_OfficeUpgrades _array_element
        (:NewEnumerator0
          (Default|CallUpgrade (.Value (Utilities|Map|Find (Variables|Default|GetMinigameList) _array_element)) :!label _label))
        (:NewEnumerator1
          (goto _label))
        (:NewEnumerator2
          (for _array_element_2 _workerdeskrefs
            (Default|DeskUpgradeEffect _array_element_2)))
        (:NewEnumerator6
          (for _array_element_3 _workerdeskrefs
            (Default|ComputerUpgradeEffect _array_element_3)))
        (:NewEnumerator3
          (goto _label))
        (:NewEnumerator4
          (goto _label))
        (:NewEnumerator5
          (goto _label))))))

(event EventBeginPlay
  (bind _workerdeskrefs (Variables|Default|GetWorkerDeskRefs))
  (bind _asbpin_game_instance (Utilities|Casting|CastToBPIN_GameInstance (Game|GetGameInstance)))
  (bind _values (Utilities|Map|Values (Variables|/Game/GameJamContent/Player/BPIN_GameInstance.BPIN_GameInstance_C|GetOfficeUpgrades _asbpin_game_instance)))
  (for _array_element _values
    (if (and (.UpgradeBought (Utilities|Struct|BreakS_OfficeUpgrades _array_element)) (.Minigame? (Utilities|Struct|BreakS_OfficeUpgrades _array_element)))
      (Variables|/Game/GameJamContent/Interactables/Office/Blueprints/BPpar_Interactables.BPpar_Interactables_C|SetUpgradeMaterial (.Value (Utilities|Map|Find (Variables|Default|GetMinigameList) (.UpgradeType (Utilities|Struct|BreakS_OfficeUpgrades _array_element)))) (.UpgradeMaterial (Utilities|Struct|BreakS_OfficeUpgrades _array_element)))
      (Variables|/Game/GameJamContent/Interactables/Office/Blueprints/BPpar_Interactables.BPpar_Interactables_C|SetUpgradeAmount (.Value (Utilities|Map|Find (Variables|Default|GetMinigameList) (.UpgradeType (Utilities|Struct|BreakS_OfficeUpgrades _array_element)))) (.UpgradeValue (Utilities|Struct|BreakS_OfficeUpgrades _array_element)))
      (Default|StartGameUpgrade (.Value (Utilities|Map|Find (Variables|Default|GetMinigameList) (.UpgradeType (Utilities|Struct|BreakS_OfficeUpgrades _array_element)))))
      (elif (.UpgradeBought (Utilities|Struct|BreakS_OfficeUpgrades _array_element))
        (switch Utilities|FlowControl|Switch|SwitchonE_OfficeUpgrades (.UpgradeType (Utilities|Struct|BreakS_OfficeUpgrades _array_element))
          (:NewEnumerator2
            (for _array_element_2 _workerdeskrefs
              (Default|DeskFunction _array_element_2)))
          (:NewEnumerator6
            (for _array_element_3 _workerdeskrefs
              (Default|ComputerFunction _array_element_3))))
        (for _array_element_4 (Variables|Default|GetWorkerRefs)
          (Default|ReceiveStats _array_element_4 "NewEnumerator0" (Math|Float|Truncate (.UpgradeValue (Utilities|Struct|BreakS_OfficeUpgrades _array_element)))))))))

(fn ConstructionScript
  (bind _returnvalue (Rendering|Material|CreateDynamicMaterialInstance (Variables|Default|GetMaterial%20Reference) "None" "None" :!class /Script/Engine.KismetMaterialLibrary))
  (Variables|Default|SetDynamic _returnvalue))