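; Dungeon chest that opens once after a hold-to-interact gauge fills, dropping items through DropableComponent.
; Box overlap with BPi_Player actors toggles the prompt; interacting starts a looping timer that fills a reused coffee machine gauge widget and spins the handle.
; HoldInteract pauses the timer and clears only the displayed bar, while leaving the box also resets progress.
; Completion plays chest animations with delayed confetti and destroys the interaction components.
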(event OnComponentBeginOverlap(Box)
  (params (OverlappedComponent :type Primitive%20Component%20Object%20Reference) (OtherActor :type Actor%20Object%20Reference) (OtherComp :type Primitive%20Component%20Object%20Reference) (OtherBodyIndex :type Integer) (bFromSweep :type Boolean) (SweepResult :type Hit%20Result%20Structure%20%28by%20ref%29))
  (if (Utilities|DoesObjectImplementInterface OtherActor "/Game/GameJamContent/Player/BPi_Player.BPi_Player_C")
    (if (not (Variables|Default|GetDone?))
      (Rendering|SetVisibility (Variables|Default|GetInteractablePopUp) true false))))

(event OnComponentEndOverlap(Box)
  (params (OverlappedComponent :type Primitive%20Component%20Object%20Reference) (OtherActor :type Actor%20Object%20Reference) (OtherComp :type Primitive%20Component%20Object%20Reference) (OtherBodyIndex :type Integer))
  (if (Utilities|DoesObjectImplementInterface OtherActor "/Game/GameJamContent/Player/BPi_Player.BPi_Player_C")
    (Rendering|SetVisibility (Variables|Default|GetInteractablePopUp) false false)
    (Rendering|SetVisibility (Variables|Default|GetGauge) false false)
    (Variables|Default|SetGaugeProgress 0.0)
    (Progress|SetPercent (Variables|/Game/GameJamContent/Interactables/Office/UI/BPW_CoffeeMachineGauge.BPW_CoffeeMachineGauge_C|GetCoffeeProgressBar (Variables|Default|GetProgressRef)) 0.0)
    (Class|KismetSystemLibrary|PauseTimer 0 "IncreaseGauge")))

(event Custom|ChestAnim
  ;[0.1248 1 0.08956] Chest Animation >:)
  (Class|GeometryCacheComponent|SetPlaybackSpeed (Variables|Default|GetChestBottom) 1.0)
  (Utilities|FlowControl|Delay 0.15)
  (Components|Activation|SetActive (Variables|Default|GetConfettiVFX) true true))

(event EventBeginPlay
  (bind _asbpw_coffee_machine_gauge (Utilities|Casting|CastToBPW_CoffeeMachineGauge (UserInterface|GetUserWidgetObject (Variables|Default|GetGauge))))
  (Variables|Default|SetProgressRef _asbpw_coffee_machine_gauge))

(event EventHoldInteract
  (params (Instigator :type Actor%20Object%20Reference))
  (if (not (Variables|Default|GetDone?))
    (Rendering|SetVisibility (Variables|Default|GetGauge) false false)
    (Rendering|SetVisibility (Variables|Default|GetInteractablePopUp) true false)
    (Progress|SetPercent (Variables|/Game/GameJamContent/Interactables/Office/UI/BPW_CoffeeMachineGauge.BPW_CoffeeMachineGauge_C|GetCoffeeProgressBar (Variables|Default|GetProgressRef)) 0.0)
    (Class|KismetSystemLibrary|PauseTimer 0 "IncreaseGauge")))

(event EventInteractwithObject
  (params (PlayerReference :type BP%20Third%20Person%20Character%20Object%20Reference))
  (Variables|Default|SetPlayerRef PlayerReference)
  (if (not (Variables|Default|GetDone?))
    (Rendering|SetVisibility (Variables|Default|GetInteractablePopUp) false false)
    (Rendering|SetVisibility (Variables|Default|GetGauge) true false)
    (Utilities|Time|SetTimerbyFunctionName 0 "IncreaseGauge" 0.05 true)))

(fn ConstructionScript)

(fn IncreaseGauge
  (bind _output_get (Variables|Default|SetGaugeProgress (+ (Variables|Default|GetGaugeProgress) 2.5)))
  (Progress|SetPercent (Variables|/Game/GameJamContent/Interactables/Office/UI/BPW_CoffeeMachineGauge.BPW_CoffeeMachineGauge_C|GetCoffeeProgressBar (Variables|Default|GetProgressRef)) (/ _output_get 1e+02))
  (Transformation|AddWorldRotation (Variables|Default|GetHandle) "-18.000000,0.000000,0.000000" false false)
  (if (>= (Variables|Default|GetGaugeProgress) 1e+02)
    (Rendering|SetVisibility (Variables|Default|GetInteractablePopUp) true false)
    (Rendering|SetVisibility (Variables|Default|GetGauge) false false)
    (Variables|Default|SetGaugeProgress 0.0)
    (Progress|SetPercent (Variables|/Game/GameJamContent/Interactables/Office/UI/BPW_CoffeeMachineGauge.BPW_CoffeeMachineGauge_C|GetCoffeeProgressBar (Variables|Default|GetProgressRef)) 0.0)
    (Class|KismetSystemLibrary|PauseTimer 0 "IncreaseGauge")
    (Default|Drops (Variables|Default|GetDropableComponent) self)
    (CallFunction|ChestAnim)
    (Variables|Default|SetDone? true)
    (Components|DestroyComponent (Variables|Default|GetBox))
    (Components|DestroyComponent (Variables|Default|GetGauge))
    (Components|DestroyComponent (Variables|Default|GetInteractablePopUp))
    (Components|DestroyComponent (Variables|Default|GetHandle))))