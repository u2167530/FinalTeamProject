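; Dungeon chain lift that the player moves between two points by interacting with its lever.
; A timeline swings the lever, then Move drives a second timeline that slides the platform forward or in reverse, with chain sounds.
; Blocker collision encloses the platform during travel and is reset per endpoint on arrival, when a FlipFlop toggles InStartPoint.
; Fall-off detection is unused, leaving the character reference for the SaveLastPosition timer unset.
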(event OnComponentEndOverlap(*NOTUSED*PlayerFallenOff)
  (params (OverlappedComponent :type Primitive%20Component%20Object%20Reference) (OtherActor :type Actor%20Object%20Reference) (OtherComp :type Primitive%20Component%20Object%20Reference) (OtherBodyIndex :type Integer))
  ;[1 1 1] *NOT USED* would be for checking if player has fallen of lift
)

(event OnComponentBeginOverlap(*NOTUSED*PlayerFallenOff)
  (params (OverlappedComponent :type Primitive%20Component%20Object%20Reference) (OtherActor :type Actor%20Object%20Reference) (OtherComp :type Primitive%20Component%20Object%20Reference) (OtherBodyIndex :type Integer) (bFromSweep :type Boolean) (SweepResult :type Hit%20Result%20Structure%20%28by%20ref%29))
  ;[1 1 1] *NOT USED* would be for checking if player has fallen of lift
)

(event Custom|Move
  (bind _startpoint (Variables|Default|GetStartPoint))
  (Audio|PlaySound2D "/Game/GameJamContent/Sounds/Sound_Design/MIXED/Chain-Lift_Start_Moving_Mixed.Chain-Lift_Start_Moving_Mixed" 1.0 1.0 0.0 0 0)
  (Utilities|FlowControl|Sequence
    (:then_0
      (Collision|SetCollisionEnabled (Variables|Default|Get+XBlockPlayer) "QueryAndPhysics")
      (Collision|SetCollisionEnabled (Variables|Default|GetEntranceCollision) "QueryAndPhysics")
      (Collision|SetCollisionEnabled (Variables|Default|Get+YBlockPlayer) "QueryAndPhysics")
      (Collision|SetCollisionEnabled (Variables|Default|Get-YBlockPlayer) "QueryAndPhysics")
      (Variables|Default|SetIsStopped? false)
      (if (Variables|Default|GetInStartPoint?)
        (bind _lerp (Timeline|Lerp PlayFromStart)
          (:Update
            (Transformation|SetRelativeLocation (Variables|Default|GetLiftPLatform) (Math|Vector|Lerp(Vector) _startpoint (+ _startpoint (Variables|Default|GetEndPoint)) _lerp) false false))
          (:Finished
            (Audio|PlaySound2D "/Game/GameJamContent/Sounds/Sound_Design/MIXED/Chain-Lift_Stop-Moving_Mixed.Chain-Lift_Stop-Moving_Mixed" 1.0 1.0 0.0 0 0)
            (Audio|Components|Audio|StopDelayed (Variables|Default|GetMotionSound) 0.5)
            (Variables|Default|SetIsStopped? true)
            (Class|KismetSystemLibrary|UnPauseTimer (Variables|Default|GetAs%20BP%20Third%20Person%20Character) "SaveLastPosition")
            (if (Variables|Default|GetInStartPoint?)
              (Collision|SetCollisionEnabled (Variables|Default|Get+XBlockPlayer) "NoCollision")
              (Collision|SetCollisionEnabled (Variables|Default|GetEntranceCollision) "NoCollision")
              (Collision|SetCollisionEnabled (Variables|Default|Get+YBlockPlayer) "NoCollision")
              (Collision|SetCollisionEnabled (Variables|Default|Get-YBlockPlayer) "NoCollision")
              (else
                (Collision|SetCollisionEnabled (Variables|Default|Get+XBlockPlayer) "QueryAndPhysics")
                (Collision|SetCollisionEnabled (Variables|Default|GetEntranceCollision) "NoCollision")
                (Collision|SetCollisionEnabled (Variables|Default|Get+YBlockPlayer) "QueryAndPhysics")
                (Collision|SetCollisionEnabled (Variables|Default|Get-YBlockPlayer) "QueryAndPhysics")))
            (Utilities|FlowControl|FlipFlop
              (:A
                (Variables|Default|SetInStartPoint? false)
                (Utilities|FlowControl|DoOnce false) ; enters at Reset
              )
              (:B
                (Variables|Default|SetInStartPoint? true)
                (Utilities|FlowControl|DoOnce false) ; enters at Reset
              ))))
        (else
          (Timeline|Lerp ReverseFromEnd))))
    (:then_1
      (Utilities|FlowControl|Delay 0.25)
      (bind _returnvalue (Audio|SpawnSound2D "/Game/GameJamContent/Sounds/Sound_Design/Dungeon_Sounds/Lift/Chain-Lift_in-motion.Chain-Lift_in-motion" 1.0 1.0 0.0 0))
      (Variables|Default|SetMotionSound _returnvalue))))

(event EventBeginPlay
  (Variables|Default|SetInStartPoint? true)
  (Components|Timeline|SetPlayRate (Variables|Default|GetLerp) (/ 1.0 (Variables|Default|GetSpeedInSeconds)))
  (Collision|SetCollisionEnabled (Variables|Default|Get+XBlockPlayer) "QueryAndPhysics")
  (Collision|SetCollisionEnabled (Variables|Default|GetEntranceCollision) "NoCollision")
  (Collision|SetCollisionEnabled (Variables|Default|Get+YBlockPlayer) "QueryAndPhysics")
  (Collision|SetCollisionEnabled (Variables|Default|Get-YBlockPlayer) "QueryAndPhysics"))

(event EventInteractwithObject
  (params (PlayerReference :type BP%20Third%20Person%20Character%20Object%20Reference))
  (if (Variables|Default|GetIsStopped?)
    (Utilities|FlowControl|DoOnce false :!label _label
      (:Completed
        (if (Variables|Default|GetInStartPoint?)
          (bind _lerp (Timeline|RotateLever PlayFromStart)
            (:Update
              (Transformation|SetRelativeRotation (Variables|Default|GetLever) (Math|Rotator|Lerp(Rotator) "0.000000,90.000000,50.000000" "0.000000,90.000000,-50.000000" _lerp) false false)
              (Utilities|FlowControl|DoOnce false
                (:Completed
                  (Utilities|FlowControl|Delay 0.25)
                  (CallFunction|Move))))
            (:Finished
              (goto _label Reset)))
          (else
            (Timeline|RotateLever ReverseFromEnd)))))))

(fn ConstructionScript)