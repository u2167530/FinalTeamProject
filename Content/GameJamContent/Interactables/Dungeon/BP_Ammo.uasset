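; BP_Ammo is an ammo pickup Blueprint that delays homing toward its target while that target's ammo is at max.
; It overrides the parent's Homing event, checking that the homing target has a valid inventory component.
; A delayed while loop polls the ammo condition every fraction of a second, then calls the parent Homing once it no longer holds.
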(event EventBeginPlay
  (|CallParentFunction) ; This node is disabled and will not be called.\nDrag off pins to build functionality.
)

(event Collision|EventActorBeginOverlap
  (params (OtherActor :type Actor%20Object%20Reference))
  (|CallParentFunction OtherActor) ; This node is disabled and will not be called.\nDrag off pins to build functionality.
)

(event EventTick
  (params (DeltaSeconds :type Float%20%28single-precision%29))
  (|CallParentFunction DeltaSeconds) ; This node is disabled and will not be called.\nDrag off pins to build functionality.
)

(event EventHoming
  (bind _inventorycomponent (Variables|/Game/GameJamContent/Player/Blueprint/BP_ThirdPersonCharacter.BP_ThirdPersonCharacter_C|GetInventoryComponent (Variables|Default|GetHomingTarget))
    (:then
      (Utilities|WhilewithDelay (== (.ammo (Variables|/Game/GameJamContent/DropsSystem/InventoryComponent.InventoryComponent_C|GetInventory _inventorycomponent)) (Variables|Default|GetMax)) 0.1
        (:Completed
          (|CallParentFunction))))
    (:else)))

(fn ConstructionScript
  (|CallParentFunction))