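; BP_Pot is a breakable dungeon pot that scatters ember pickups or effects when destroyed.
; Any damage lowers its health, clamped between zero and its maximum.
; At zero health it spawns a random small number of BP_Embers actors at its own transform, then destroys itself.
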(event Game|Damage|EventAnyDamage
  (params (Damage :type Float%20%28single-precision%29) (DamageType :type Damage%20Type%20Object%20Reference) (InstigatedBy :type Controller%20Object%20Reference) (DamageCauser :type Actor%20Object%20Reference))
  ;[0.05098 0.05098 0.05098] PotBreak
  (Variables|Default|SetCurrentHealth (Math|Float|Clamp(Float) (- (Variables|Default|GetCurrentHealth) Damage) 0.0 (Variables|Default|GetMaxHealth)))
  (if (<= (Variables|Default|GetCurrentHealth) 0.0)
    (for _index (range 0 (Math|Random|RandomIntegerinRange 0 4))
      (Game|SpawnActorfromClass "/Game/GameJamContent/Interactables/Dungeon/BP_Embers.BP_Embers_C" (Transformation|GetActorTransform) "Undefined" "MultiplyWithRoot" 0 0))
    (Actor|DestroyActor)))

(event Collision|EventActorBeginOverlap
  (params (OtherActor :type Actor%20Object%20Reference)))

(event EventTick
  (params (DeltaSeconds :type Float%20%28single-precision%29)))

(event EventBeginPlay)

(fn ConstructionScript)