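; Lever-operated dungeon lift that can pair with a fellow lift to teleport the player between platforms.
; Interacting while inside animates the lever and calls Move on both lifts, running a timeline between start and end points with blocking colliders and optional sounds.
; TeleportCollision overlap fades the camera and places the player on the fellow platform at the same XY offset, briefly disabling its trigger.
; Move also suspends the LifeSteal pickup during travel.
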(event OnComponentBeginOverlap(InteractCollision)
  (params (OverlappedComponent :type Primitive%20Component%20Object%20Reference) (OtherActor :type Actor%20Object%20Reference) (OtherComp :type Primitive%20Component%20Object%20Reference) (OtherBodyIndex :type Integer) (bFromSweep :type Boolean) (SweepResult :type Hit%20Result%20Structure%20%28by%20ref%29))
  (if (Utilities|DoesObjectImplementInterface OtherActor "/Game/GameJamContent/Player/BPi_Player.BPi_Player_C")
    (if (Variables|Default|GetIsStopped?)
      (Utilities|FlowControl|DoOnce false
        (:Completed
          (Variables|Default|Setplayerininteract true)
          (Rendering|SetVisibility (Variables|Default|GetEtoInteract) true false)
          (Utilities|FlowControl|DoOnce false) ; enters at Reset
        )))))

(event OnComponentBeginOverlap(TeleportCollision)
  (params (OverlappedComponent :type Primitive%20Component%20Object%20Reference) (OtherActor :type Actor%20Object%20Reference) (OtherComp :type Primitive%20Component%20Object%20Reference) (OtherBodyIndex :type Integer) (bFromSweep :type Boolean) (SweepResult :type Hit%20Result%20Structure%20%28by%20ref%29))
  (bind _returnvalue (Transformation|GetActorLocation))
  (bind _fellowliftref (Variables|Default|GetFellowLiftRef))
  (bind _as_bp_third_person_character (Variables|Default|GetAs%20BP%20Third%20Person%20Character))
  (bind _as_bp_third_person_character_2 (Variables|Default|GetAs%20BP%20Third%20Person%20Character))
  (bind _returnvalue_2 (Transformation|GetActorLocation _as_bp_third_person_character))
  (bind _liftplatform (Variables|BP_LiftWithTeleport_C|GetLiftPLatform _fellowliftref))
  (bind _returnvalue_3 (Transformation|GetWorldLocation _liftplatform))
  (bind _returnvalue_4 (- (.y _returnvalue_2) (.y _returnvalue)))
  (bind _returnvalue_5 (- (.x _returnvalue_2) (.x _returnvalue)))
  (bind _returnvalue_6 (Math|Vector|MakeVector _returnvalue_5 _returnvalue_4 0.0))
  (bind _returnvalue_7 (+ _returnvalue_3 _returnvalue_6))
  (if (Utilities|DoesObjectImplementInterface OtherActor "/Game/GameJamContent/Player/BPi_Player.BPi_Player_C")
    (Utilities|IsValid (Variables|Default|GetFellowLiftRef)
      (:Is%20Valid
        (Utilities|FlowControl|DoOnce false :!label _label
          (:Completed
            (Collision|SetCollisionEnabled (Variables|BP_LiftWithTeleport_C|GetTeleportCollision (Variables|Default|GetFellowLiftRef)) "NoCollision")
            (CameraFades|StartCameraFade (Variables|/Script/Engine.PlayerController|GetPlayerCameraManager (Game|GetPlayerController 0)) 0.0 1.0 1.0 "(R=0.000000,G=0.000000,B=0.000000,A=1.000000)" false true)
            (Utilities|FlowControl|Delay 1.0)
            (if (Variables|Default|GetInStartPoint?)
              (Transformation|SetActorLocation _as_bp_third_person_character_2 (+ _returnvalue_7 "0.000000,0.000000,100.000000") false false)
              (else
                (Transformation|SetActorLocation _as_bp_third_person_character_2 (+ _returnvalue_7 "0.000000,0.000000,100.000000") false false)))
            (Utilities|FlowControl|Delay 1.0)
            (CameraFades|StartCameraFade :self (Variables|/Script/Engine.PlayerController|GetPlayerCameraManager (Game|GetPlayerController 0)) :FromAlpha 1.0 :Duration 2.0)
            (Utilities|FlowControl|Delay 0.2)
            (Collision|SetCollisionEnabled (Variables|BP_LiftWithTeleport_C|GetTeleportCollision (Variables|Default|GetFellowLiftRef)) "QueryAndPhysics")
            (goto _label Reset)))))))

(event OnComponentEndOverlap(PlayerRefCollision)
  (params (OverlappedComponent :type Primitive%20Component%20Object%20Reference) (OtherActor :type Actor%20Object%20Reference) (OtherComp :type Primitive%20Component%20Object%20Reference) (OtherBodyIndex :type Integer))
  (if (Utilities|DoesObjectImplementInterface OtherActor "/Game/GameJamContent/Player/BPi_Player.BPi_Player_C")
    (Utilities|FlowControl|DoOnce false
      (:Completed
        (Variables|Default|SetIsPlayerInside? false)
        (Utilities|FlowControl|DoOnce false) ; enters at Reset
      ))))

(event OnComponentBeginOverlap(PlayerRefCollision)
  (params (OverlappedComponent :type Primitive%20Component%20Object%20Reference) (OtherActor :type Actor%20Object%20Reference) (OtherComp :type Primitive%20Component%20Object%20Reference) (OtherBodyIndex :type Integer) (bFromSweep :type Boolean) (SweepResult :type Hit%20Result%20Structure%20%28by%20ref%29))
  (if (Utilities|DoesObjectImplementInterface OtherActor "/Game/GameJamContent/Player/BPi_Player.BPi_Player_C")
    (Utilities|FlowControl|DoOnce false
      (:Completed
        (Variables|Default|SetIsPlayerInside? true)
        (Utilities|FlowControl|DoOnce false) ; enters at Reset
      ))))

(event OnComponentEndOverlap(InteractCollision)
  (params (OverlappedComponent :type Primitive%20Component%20Object%20Reference) (OtherActor :type Actor%20Object%20Reference) (OtherComp :type Primitive%20Component%20Object%20Reference) (OtherBodyIndex :type Integer))
  (if (Utilities|DoesObjectImplementInterface OtherActor "/Game/GameJamContent/Player/BPi_Player.BPi_Player_C")
    (if (Variables|Default|GetIsStopped?)
      (Utilities|FlowControl|DoOnce false
        (:Completed
          (Variables|Default|Setplayerininteract false)
          (Rendering|SetVisibility (Variables|Default|GetEtoInteract) false false)
          (Utilities|FlowControl|DoOnce false) ; enters at Reset
        )))))

(event Custom|Move
  (bind _startpoint (Variables|Default|GetStartPoint))
  (bind _as_bp_third_person_character (Variables|Default|GetAs%20BP%20Third%20Person%20Character))
  (bind _as_bp_third_person_character_2 (Variables|Default|GetAs%20BP%20Third%20Person%20Character))
  (if (Variables|Default|GetPlaySound)
    (Audio|PlaySound2D "/Game/GameJamContent/Sounds/Sound_Design/MIXED/Chain-Lift_Start_Moving_Mixed.Chain-Lift_Start_Moving_Mixed" 1.0 1.0 0.0 0 0))
  (Utilities|FlowControl|Sequence
    (:then_0
      (Collision|SetCollisionEnabled (Variables|Default|Get+XBlockPlayer) "QueryAndPhysics")
      (Collision|SetCollisionEnabled (Variables|Default|Get-XBlockPlayer) "QueryAndPhysics")
      (Collision|SetCollisionEnabled (Variables|Default|Get+YBlockPlayer) "QueryAndPhysics")
      (Collision|SetCollisionEnabled (Variables|Default|Get-YBlockPlayer) "QueryAndPhysics")
      (Rendering|SetVisibility (Variables|Default|GetEtoInteract) false false)
      (CallFunction|ResetDoOnce)
      (if (Utilities|Array|ContainsItem (Variables|/Game/GameJamContent/Player/Blueprint/BP_ThirdPersonCharacter.BP_ThirdPersonCharacter_C|GetPicked _as_bp_third_person_character_2) 2)
        (Default|BreakLifeSteal _as_bp_third_person_character_2))
      (Variables|Default|SetIsStopped? false)
      (if (Variables|Default|GetInStartPoint?)
        (bind _lerp (Timeline|Lerp PlayFromStart)
          (:Update
            (Transformation|SetRelativeLocation (Variables|Default|GetLiftPLatform) (Math|Vector|Lerp(Vector) _startpoint (+ _startpoint (Variables|Default|GetEndPoint)) _lerp) false false))
          (:Finished
            (if (Variables|Default|GetPlaySound)
              (Audio|PlaySound2D "/Game/GameJamContent/Sounds/Sound_Design/MIXED/Chain-Lift_Stop-Moving_Mixed.Chain-Lift_Stop-Moving_Mixed" 1.0 1.0 0.0 0 0)
              (Audio|Components|Audio|StopDelayed (Variables|Default|GetMotionSound) 0.5))
            (if (Utilities|Array|ContainsItem (Variables|/Game/GameJamContent/Player/Blueprint/BP_ThirdPersonCharacter.BP_ThirdPersonCharacter_C|GetPicked _as_bp_third_person_character) 2)
              (Default|LifeSteal _as_bp_third_person_character))
            (Variables|Default|SetIsStopped? true)
            (Collision|SetCollisionEnabled (Variables|Default|Get+XBlockPlayer) "NoCollision")
            (Collision|SetCollisionEnabled (Variables|Default|Get-XBlockPlayer) "NoCollision")
            (Collision|SetCollisionEnabled (Variables|Default|Get+YBlockPlayer) "NoCollision")
            (Collision|SetCollisionEnabled (Variables|Default|Get-YBlockPlayer) "NoCollision")
            (Utilities|FlowControl|FlipFlop
              (:A
                (Variables|Default|SetInStartPoint? false))
              (:B
                (Variables|Default|SetInStartPoint? true)))))
        (else
          (Timeline|Lerp ReverseFromEnd))))
    (:then_1
      (Utilities|FlowControl|Delay 0.25)
      (if (Variables|Default|GetPlaySound)
        (bind _returnvalue (Audio|SpawnSound2D "/Game/GameJamContent/Sounds/Sound_Design/Dungeon_Sounds/Lift/Chain-Lift_in-motion.Chain-Lift_in-motion" 0.6 1.0 0.0 0))
        (Variables|Default|SetMotionSound _returnvalue)))))

(event Custom|ResetDoOnce
  (Utilities|FlowControl|Sequence
    (:then_0
      (Utilities|FlowControl|DoOnce false) ; enters at Reset
    )
    (:then_1
      (Utilities|FlowControl|DoOnce false) ; enters at Reset
    )))

(event EventBeginPlay
  (Variables|Default|SetInStartPoint? true)
  (Components|Timeline|SetPlayRate (Variables|Default|GetLerp) (/ 1.0 (Variables|Default|GetSpeedInSeconds)))
  (Collision|SetCollisionEnabled (Variables|Default|Get+XBlockPlayer) "NoCollision")
  (Collision|SetCollisionEnabled (Variables|Default|Get-XBlockPlayer) "NoCollision")
  (Collision|SetCollisionEnabled (Variables|Default|Get+YBlockPlayer) "NoCollision")
  (Collision|SetCollisionEnabled (Variables|Default|Get-YBlockPlayer) "NoCollision")
  (bind _asbp_third_person_character (Utilities|Casting|CastToBP_ThirdPersonCharacter (Game|GetPlayerCharacter 0)))
  (Variables|Default|SetAs%20BP%20Third%20Person%20Character _asbp_third_person_character))

(event EventInteractwithObject
  (params (PlayerReference :type BP%20Third%20Person%20Character%20Object%20Reference))
  (bind _fellowliftref (Variables|Default|GetFellowLiftRef))
  (Variables|Default|SetAs%20BP%20Third%20Person%20Character PlayerReference)
  (if (Variables|Default|GetIsPlayerInside?)
    (if (Variables|Default|GetIsStopped?)
      (Utilities|FlowControl|DoOnce false :!label _label
        (:Completed
          (if (Variables|Default|GetInStartPoint?)
            (bind _lerp (Timeline|Timeline PlayFromStart)
              (:Update
                (Transformation|SetRelativeRotation (Variables|Default|GetLever) (Math|Rotator|Lerp(Rotator) "0.000000,90.000000,50.000000" "0.000000,90.000000,-50.000000" _lerp) false false)
                (Utilities|FlowControl|DoOnce false
                  (:Completed
                    (Utilities|FlowControl|Delay 0.25)
                    (CallFunction|Move)
                    (Utilities|IsValid _fellowliftref
                      (:Is%20Valid
                        (Variables|BP_LiftWithTeleport_C|SetAs%20BP%20Third%20Person%20Character _fellowliftref (Variables|Default|GetAs%20BP%20Third%20Person%20Character))
                        (CallFunction|Move _fellowliftref))))))
              (:Finished
                (goto _label Reset)))
            (else
              (Timeline|Timeline ReverseFromEnd))))))))

(fn ConstructionScript
  (Transformation|SetRelativeLocation (Variables|Default|GetTeleportCollision) (Variables|Default|GetTeleportLocation) false false))