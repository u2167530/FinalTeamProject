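; BP_Checkpoint is an interactable dungeon checkpoint that pauses the game and opens the checkpoint menu when a player uses it.
; On interaction with a valid player, it creates BPW_Checkpoint and adds it to the viewport.
; The widget receives a snapshot of the player's dungeon HUD state (contract progress, worker happiness, office time), inventory Embers and location, flagged as coming from a checkpoint.
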(event EventInteractwithObject
  (params (PlayerReference :type BP%20Third%20Person%20Character%20Object%20Reference))
  (bind _dungeonhudreference (Variables|/Game/GameJamContent/Player/Blueprint/BP_ThirdPersonCharacter.BP_ThirdPersonCharacter_C|GetDungeonHUDReference PlayerReference))
  (Utilities|IsValid PlayerReference
    (:Is%20Valid
      (Game|SetGamePaused true)
      (bind _returnvalue (UserInterface|CreateWidget "/Game/GameJamContent/Interactables/Dungeon/Checkpoint/BPW_Checkpoint.BPW_Checkpoint_C" 0 (Variables|/Game/GameJamContent/Player/UI/BPW_DungeonHUD.BPW_DungeonHUD_C|GetContractProgress _dungeonhudreference) (Variables|/Game/GameJamContent/Player/UI/BPW_DungeonHUD.BPW_DungeonHUD_C|GetWorkerHappiness _dungeonhudreference) (Variables|/Game/GameJamContent/Player/UI/BPW_DungeonHUD.BPW_DungeonHUD_C|GetContractPercent _dungeonhudreference) (Variables|/Game/GameJamContent/Player/UI/BPW_DungeonHUD.BPW_DungeonHUD_C|GetOfficeTime _dungeonhudreference) (Variables|/Game/GameJamContent/Player/UI/BPW_DungeonHUD.BPW_DungeonHUD_C|GetIsAM _dungeonhudreference) (.embers (Variables|/Game/GameJamContent/DropsSystem/InventoryComponent.InventoryComponent_C|GetInventory (Variables|/Game/GameJamContent/Player/Blueprint/BP_ThirdPersonCharacter.BP_ThirdPersonCharacter_C|GetInventoryComponent PlayerReference))) (Transformation|GetActorLocation PlayerReference) true))
      (UserInterface|Viewport|AddtoViewport _returnvalue 0))))

(fn ConstructionScript)