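; A dungeon moving platform that shuttles between its start point and an end offset when the player steps on its trigger.
; A Lerp timeline, rate-scaled by SpeedInSeconds, moves the Cube, alternating direction each trip and also starting an optional linked FellowLiftRef.
; The player's SaveLastPosition timer pauses during the ride.
; Falling out of the outer volume mid-ride resumes that timer and snaps the platform back after a delay.
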(event OnComponentBeginOverlap(startmovement)
  (params (OverlappedComponent :type Primitive%20Component%20Object%20Reference) (OtherActor :type Actor%20Object%20Reference) (OtherComp :type Primitive%20Component%20Object%20Reference) (OtherBodyIndex :type Integer) (bFromSweep :type Boolean) (SweepResult :type Hit%20Result%20Structure%20%28by%20ref%29))
  (bind _fellowliftref (Variables|Default|GetFellowLiftRef))
  (if (Utilities|DoesObjectImplementInterface OtherActor "/Game/GameJamContent/Player/BPi_Player.BPi_Player_C")
    (if (Variables|Default|GetIsStopped?)
      (Class|KismetSystemLibrary|PauseTimer (Variables|Default|GetAs%20BP%20Third%20Person%20Character) "SaveLastPosition")
      (CallFunction|Move)
      (Utilities|IsValid _fellowliftref
        (:Is%20Valid
          (Variables|BP_MovingPlatform1_C|SetAs%20BP%20Third%20Person%20Character _fellowliftref (Variables|Default|GetAs%20BP%20Third%20Person%20Character))
          (CallFunction|Move _fellowliftref))))))

(event OnComponentEndOverlap(PlayerFallenOff)
  (params (OverlappedComponent :type Primitive%20Component%20Object%20Reference) (OtherActor :type Actor%20Object%20Reference) (OtherComp :type Primitive%20Component%20Object%20Reference) (OtherBodyIndex :type Integer))
  (if (Utilities|DoesObjectImplementInterface OtherActor "/Game/GameJamContent/Player/BPi_Player.BPi_Player_C")
    (if (AI|Components|NavMovement|IsFalling (Variables|/Script/Engine.Character|GetCharacterMovement (Variables|Default|GetAs%20BP%20Third%20Person%20Character)))
      (Class|KismetSystemLibrary|UnPauseTimer (Variables|Default|GetAs%20BP%20Third%20Person%20Character) "SaveLastPosition")
      (if (not (Variables|Default|GetIsStopped?))
        (Audio|Components|Audio|Stop (Variables|Default|GetLerp))
        (Utilities|FlowControl|Delay 1.0)
        (if (Variables|Default|GetInStartPoint?)
          (Transformation|SetRelativeLocation (Variables|Default|GetCube) "0, 0, 0" false false)
          (Variables|Default|SetInStartPoint? true)
          (else
            (Transformation|SetRelativeLocation (Variables|Default|GetCube) (Variables|Default|GetEndPoint) false false)
            (Variables|Default|SetInStartPoint? false)))
        (Variables|Default|SetIsStopped? true)))))

(event OnComponentBeginOverlap(PlayerFallenOff)
  (params (OverlappedComponent :type Primitive%20Component%20Object%20Reference) (OtherActor :type Actor%20Object%20Reference) (OtherComp :type Primitive%20Component%20Object%20Reference) (OtherBodyIndex :type Integer) (bFromSweep :type Boolean) (SweepResult :type Hit%20Result%20Structure%20%28by%20ref%29))
  (if (Utilities|DoesObjectImplementInterface OtherActor "/Game/GameJamContent/Player/BPi_Player.BPi_Player_C")
    (bind _asbp_third_person_character (Utilities|Casting|CastToBP_ThirdPersonCharacter OtherActor))
    (Variables|Default|SetAs%20BP%20Third%20Person%20Character _asbp_third_person_character)))

(event Custom|Move
  (bind _startpoint (Variables|Default|GetStartPoint))
  (Variables|Default|SetIsStopped? false)
  (if (Variables|Default|GetInStartPoint?)
    (bind _lerp (Timeline|Lerp PlayFromStart)
      (:Update
        (Transformation|SetRelativeLocation (Variables|Default|GetCube) (Math|Vector|Lerp(Vector) _startpoint (+ _startpoint (Variables|Default|GetEndPoint)) _lerp) false false))
      (:Finished
        (Variables|Default|SetIsStopped? true)
        (Class|KismetSystemLibrary|UnPauseTimer (Variables|Default|GetAs%20BP%20Third%20Person%20Character) "SaveLastPosition")
        (Utilities|FlowControl|FlipFlop
          (:A
            (Variables|Default|SetInStartPoint? false))
          (:B
            (Variables|Default|SetInStartPoint? true)))))
    (else
      (Timeline|Lerp ReverseFromEnd))))

(event EventBeginPlay
  (Variables|Default|SetInStartPoint? true)
  (Components|Timeline|SetPlayRate (Variables|Default|GetLerp) (/ 1.0 (Variables|Default|GetSpeedInSeconds))))

(fn ConstructionScript)