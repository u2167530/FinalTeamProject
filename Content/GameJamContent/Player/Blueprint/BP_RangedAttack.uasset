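; BP_RangedAttack is a short-lived physics projectile that explodes on impact, usable by the player or against them via the FromPlayer flag.
; Tick applies a strong custom downward acceleration to the Sphere.
; Physical hits, or HitBox overlaps with valid targets, trigger a one-time explosion that scales effect and radius by Size, halts the projectile, then destroys it.
; The Explosion overlap sends damage only to the first valid target.
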(event OnComponentBeginOverlap(HitBox)
  (params (OverlappedComponent :type Primitive%20Component%20Object%20Reference) (OtherActor :type Actor%20Object%20Reference) (OtherComp :type Primitive%20Component%20Object%20Reference) (OtherBodyIndex :type Integer) (bFromSweep :type Boolean) (SweepResult :type Hit%20Result%20Structure%20%28by%20ref%29))
  (if (and (Utilities|DoesObjectImplementInterface OtherActor "/Game/GameJamContent/Player/BPi_Player.BPi_Player_C") (not (Variables|Default|GetFromPlayer)))
    (CallFunction|Explode)
    (elif (and (Actor|ActorHasTag OtherActor "CanTakeDamage") (Variables|Default|GetFromPlayer))
      (CallFunction|Explode))))

(event OnComponentHit(Sphere)
  (params (HitComponent :type Primitive%20Component%20Object%20Reference) (OtherActor :type Actor%20Object%20Reference) (OtherComp :type Primitive%20Component%20Object%20Reference) (NormalImpulse :type Vector :default "0, 0, 0") (Hit :type Hit%20Result%20Structure%20%28by%20ref%29))
  (CallFunction|Explode))

(event OnComponentBeginOverlap(Explosion)
  (params (OverlappedComponent :type Primitive%20Component%20Object%20Reference) (OtherActor :type Actor%20Object%20Reference) (OtherComp :type Primitive%20Component%20Object%20Reference) (OtherBodyIndex :type Integer) (bFromSweep :type Boolean) (SweepResult :type Hit%20Result%20Structure%20%28by%20ref%29))
  (if (and (Actor|ActorHasTag OtherActor "CanTakeDamage") (Variables|Default|GetFromPlayer))
    (Utilities|FlowControl|DoOnce false :!label _label
      (:Completed
        (Class|BPIDamageable|TakeDamage(Message) OtherActor (Utilities|Struct|MakeS_DamageInfo 1e+01 "NewEnumerator2" "NewEnumerator1" false))))
    (elif (and (Utilities|DoesObjectImplementInterface OtherActor "/Game/GameJamContent/Player/BPi_Player.BPi_Player_C") (not (Variables|Default|GetFromPlayer)))
      (goto _label))))

(event Custom|Explode
  (bind _sphere (Variables|Default|GetSphere))
  (bind _explosion (Variables|Default|GetExplosion))
  (bind _size (Variables|Default|GetSize))
  (Utilities|FlowControl|DoOnce false
    (:Completed
      (Effects|SpawnEmitteratLocation "/Game/StarterContent/Particles/P_Explosion.P_Explosion" (Transformation|GetActorLocation) "0, 0, 0" (Math|Vector|MakeVector _size _size _size))
      (Components|Sphere|SetSphereRadius _explosion (* (Variables|/Script/Engine.SphereComponent|GetSphereRadius _explosion) (Variables|Default|GetSize)) true)
      (Collision|SetCollisionEnabled _explosion "QueryAndPhysics")
      ;[1 1 1] Stops projectile from moving after it hits something
      (Rendering|SetVisibility _sphere false false)
      (Physics|SetEnableGravity _sphere false)
      (Physics|SetPhysicsLinearVelocity _sphere "0, 0, 0" false "None")
      (Utilities|FlowControl|Delay 1.0)
      (Actor|DestroyActor))))

(event EventBeginPlay
  (Actor|SetLifeSpan 2.0))

(event EventTick
  (params (DeltaSeconds :type Float%20%28single-precision%29))
  (bind _sphere (Variables|Default|GetSphere))
  (Physics|AddForce _sphere (* (Math|Vector|MakeVector 0.0 0.0 (* (Math|Float|MakeLiteralFloat -9.8) (Math|Float|MakeLiteralFloat 3e+02))) (Math|Vector|GetUpVector _sphere)) "None" true))

(fn ConstructionScript)