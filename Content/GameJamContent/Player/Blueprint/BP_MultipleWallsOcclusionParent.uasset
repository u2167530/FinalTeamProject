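; Parent actor for groups of walls that can be switched to occlusion materials and back, judging by its name and events.
; On BeginPlay it caches every primitive component and its slot 0 material.
; TurnInvis finds each material's "OP"-suffixed counterpart by name in the supplied asset array, applies it and makes the component ignore the Visibility channel.
; TurnVis restores the cached materials and Visibility blocking.
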(event Custom|TurnInvis
  (params (Array :type Array%20of%20Asset%20Data%20Structures))
  (for _array_element (Variables|Default|GetCOM)
    (bind _array_element_2 (Utilities|Array|ForEachLoopwithBreak Array :!label _label)
      (:LoopBody
        (if (== (.AssetName (Utilities|Struct|BreakAssetData _array_element_2)) (Utilities|String|Append (Utilities|GetObjectName (Rendering|Material|GetMaterial _array_element 0)) "OP"))
          (goto _label Break)))
      (:Completed
        (bind _asmaterial_interface (Utilities|Casting|CastToMaterialInterface (Class|AssetRegistryHelpers|GetAsset _array_element_2)))
        (Rendering|Material|SetMaterial _array_element 0 _asmaterial_interface)
        (Collision|SetCollisionResponsetoChannel _array_element "ECC_Visibility" "ECR_Ignore")))))

(event Custom|TurnVis
  (for (_array_element _array_index) (Variables|Default|GetCOM)
    (Rendering|Material|SetMaterial _array_element 0 (Utilities|Array|Get(acopy) (Variables|Default|GetMaterials) _array_index))
    (Collision|SetCollisionResponsetoChannel _array_element "ECC_Visibility" "ECR_Block")))

(event EventBeginPlay
  (bind _output_get (Variables|Default|SetCOM (Actor|GetComponentsByClass "/Script/Engine.PrimitiveComponent")))
  (for _array_element _output_get
    (Utilities|Array|Add (Variables|Default|GetMaterials) (Rendering|Material|GetMaterial _array_element 0))))

(event Collision|EventActorBeginOverlap
  (params (OtherActor :type Actor%20Object%20Reference)))

(event EventTick
  (params (DeltaSeconds :type Float%20%28single-precision%29)))

(fn ConstructionScript)