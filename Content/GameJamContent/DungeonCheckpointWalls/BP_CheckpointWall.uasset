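; BP_CheckpointWall is a dungeon checkpoint wall that destroys itself when its spawn stage is cleared of enemies.
; The construction script finds BP_SpawnController and binds to its NoEnemies event.
; On that event, the wall compares its SpawnIndex to the controller's index minus one and, on a match, prints a debug string and destroys itself.
; Player-overlap visibility and kill-count text logic for a widget is present but disconnected.
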(event OnComponentBeginOverlap(Box)
  (params (OverlappedComponent :type Primitive%20Component%20Object%20Reference) (OtherActor :type Actor%20Object%20Reference) (OtherComp :type Primitive%20Component%20Object%20Reference) (OtherBodyIndex :type Integer) (bFromSweep :type Boolean) (SweepResult :type Hit%20Result%20Structure%20%28by%20ref%29)))

(event OnComponentEndOverlap(Box)
  (params (OverlappedComponent :type Primitive%20Component%20Object%20Reference) (OtherActor :type Actor%20Object%20Reference) (OtherComp :type Primitive%20Component%20Object%20Reference) (OtherBodyIndex :type Integer)))

(event Custom|NoEnemies
  (bind _returnvalue (Actor|GetActorOfClass "/Game/GameJamContent/SpawnSystem/BP_SpawnController.BP_SpawnController_C"))
  (if (== (Variables|Default|GetSpawnIndex) (- (Variables|/Game/GameJamContent/SpawnSystem/BP_SpawnController.BP_SpawnController_C|GetSpawnIndex _returnvalue) 1))
    (Development|PrintString "Hello")
    (Actor|DestroyActor)))

(event EventBeginPlay)

(fn ConstructionScript
  (bind _returnvalue (Actor|GetActorOfClass "/Game/GameJamContent/SpawnSystem/BP_SpawnController.BP_SpawnController_C"))
  (bind _output_get (Variables|Default|SetSpawnControllerRef _returnvalue))
  (EventDispatchers|BindEventtoNoEnemies _output_get (EventDispatchers|CreateEvent :!event Custom|NoEnemies)))