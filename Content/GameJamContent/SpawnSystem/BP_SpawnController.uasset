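; BP_SpawnController runs wave-based enemy spawning, starting the first wave shortly after BeginPlay by calling Spawn.
; A few seconds after each Spawn call, it counts the BP_Enemy1 actors in the level, printing the running count.
; ReduceEnemyCount decrements that count and fires NoEnemies at zero.
; The handler, bound in the construction script, increments SpawnIndex, calls Spawn again and repeats the delayed count.
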(event Custom|NoEnemies_Event
  (CallFunction|SpawnCurrentIndex)
  (Utilities|FlowControl|Delay 3.0)
  (bind _outactors (Actor|GetAllActorsOfClass "/Game/GameJamContent/Enemy/Standard/BP_Enemy1.BP_Enemy1_C"))
  (Variables|Default|SetEnemycount 0)
  (for _array_element _outactors
    (bind _output_get (Variables|Default|SetEnemycount (+ (Variables|Default|GetEnemycount) 1)))
    (Development|PrintString (Utilities|String|ToString(Integer) _output_get))))

(event EventBeginPlay
  (Utilities|FlowControl|Delay 0.2)
  (Default|CallSpawn)
  (Utilities|FlowControl|Delay 3.0)
  (bind _outactors (Actor|GetAllActorsOfClass "/Game/GameJamContent/Enemy/Standard/BP_Enemy1.BP_Enemy1_C"))
  (Variables|Default|SetEnemycount 0)
  (for _array_element _outactors
    (bind _output_get (Variables|Default|SetEnemycount (+ (Variables|Default|GetEnemycount) 1)))
    (Development|PrintString (Utilities|String|ToString(Integer) _output_get))))

(event EventTick
  (params (DeltaSeconds :type Float%20%28single-precision%29)))

(event Collision|EventActorBeginOverlap
  (params (OtherActor :type Actor%20Object%20Reference)))

(fn ConstructionScript
  (EventDispatchers|BindEventtoNoEnemies (EventDispatchers|CreateEvent :!event Custom|NoEnemies_Event)))

(fn SpawnCurrentIndex
  (Variables|Default|SetSpawnIndex (+ (Variables|Default|GetSpawnIndex) 1))
  (Default|CallSpawn)
  (return))

(fn ReduceEnemyCount
  (Variables|Default|SetEnemycount (- (Variables|Default|GetEnemycount) 1))
  (if (<= (Variables|Default|GetEnemycount) 0)
    (Default|CallNoEnemies))
  (return))