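; BP_WallRepeater is a dungeon environment actor that builds a straight wall from repeated mesh tiles.
; Its construction script divides XValue's X by Length to set the tile count, adding static mesh components spaced along local X.
; BrickOrNah switches the base WallTile between brick and rock meshes.
; Repeated brick tiles randomly pick one of three variations on each construction, while rock tiles keep the added component's default mesh.
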(event EventBeginPlay)

(event Collision|EventActorBeginOverlap
  (params (OtherActor :type Actor%20Object%20Reference)))

(event EventTick
  (params (DeltaSeconds :type Float%20%28single-precision%29)))

(fn ConstructionScript
  (if (Variables|Default|GetBrickOrNah)
    (Components|StaticMesh|SetStaticMesh (Variables|Default|GetWallTile) "/Game/GameJamContent/Environment/Dungeon/FBX_Models/SM_Dungeon_BrickWallVariation2.SM_Dungeon_BrickWallVariation2")
    (else
      (Components|StaticMesh|SetStaticMesh (Variables|Default|GetWallTile) "/Game/GameJamContent/Environment/Dungeon/FBX_Models/SM_Dungeon_RockWallBase.SM_Dungeon_RockWallBase")))
  (for _index (range 0 (Math|Float|Truncate (/ (.x (Variables|Default|GetXValue)) (Variables|Default|GetLength))))
    (if (Variables|Default|GetBrickOrNah)
      (bind _returnvalue (AddComponent|AddStaticMeshComponent false (Math|Transform|MakeTransform (Math|Vector|MakeVector (* _index (Variables|Default|GetLength)) 0.0 0.0) (Math|Rotator|MakeRotator 0.0 0.0 0.0) "1.000000,1.000000,1.000000")))
      (Components|StaticMesh|SetStaticMesh _returnvalue (Utilities|Select :Index (Math|Random|RandomInteger 3) :Option%200 "/Game/GameJamContent/Environment/Dungeon/FBX_Models/SM_Dungeon_BrickWallVariation1.SM_Dungeon_BrickWallVariation1" :Option%201 "/Game/GameJamContent/Environment/Dungeon/FBX_Models/SM_Dungeon_BrickWallVariation2.SM_Dungeon_BrickWallVariation2" :Option%202 "/Game/GameJamContent/Environment/Dungeon/FBX_Models/SM_Dungeon_BrickWallVariation3.SM_Dungeon_BrickWallVariation3"))
      (else
        (AddComponent|AddStaticMeshComponent false (Math|Transform|MakeTransform (Math|Vector|MakeVector (* _index (Variables|Default|GetLength)) 0.0 0.0) (Math|Rotator|MakeRotator 0.0 0.0 0.0) "1.000000,1.000000,1.000000"))))))