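; BP_CircusTent is a circus tent environment Blueprint whose top can be removed and added back at runtime.
; The RemopveTop event destroys the CircusTop component, and AddTop creates a new static mesh component and stores it as CircusTop.
; A HasTop flag guards both events so the top is never removed or added twice in a row.
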(event Custom|RemopveTop
  (if (Variables|Default|GetHasTop?)
    (Components|DestroyComponent (Variables|Default|GetCircusTop))
    (Variables|Default|SetHasTop? false)))

(event Custom|AddTop
  (if (not (Variables|Default|GetHasTop?))
    (bind _returnvalue (AddComponent|AddStaticMeshComponent false))
    (Variables|Default|SetCircusTop _returnvalue)
    (Variables|Default|SetHasTop? true)))

(fn ConstructionScript)