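; BP_RailingRepeater is a dungeon environment actor that builds a repeating railing along its local X axis.
; Its construction script divides XValue.X by Length to get the piece count, then adds static mesh components at Length intervals.
; Each step pairs a base piece with a scaled, Y-offset piece, likely a post, and one extra offset piece caps the end.
; The event graph is empty.
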(event EventBeginPlay)

(event Collision|EventActorBeginOverlap
  (params (OtherActor :type Actor%20Object%20Reference)))

(event EventTick
  (params (DeltaSeconds :type Float%20%28single-precision%29)))

(fn ConstructionScript
  (bind _xvalue (Variables|Default|GetXValue))
  (bind _length (Variables|Default|GetLength))
  (bind _returnvalue (/ (.x _xvalue) _length))
  (bind _returnvalue_2 (Math|Float|Truncate _returnvalue))
  (Components|StaticMesh|SetStaticMesh (Variables|Default|GetWallTile) "/Game/GameJamContent/Environment/Dungeon/FBX_Models/SM_Dungeon_BrickRailing.SM_Dungeon_BrickRailing")
  (for _index (range 0 _returnvalue_2)
    (AddComponent|AddStaticMeshComponent false (Math|Transform|MakeTransform (Math|Vector|MakeVector (* _index (Variables|Default|GetLength)) 0.0 0.0) (Math|Rotator|MakeRotator 0.0 0.0 0.0) "1.000000,1.000000,1.000000"))
    (bind _returnvalue_3 (AddComponent|AddStaticMeshComponent false (Math|Transform|MakeTransform (Math|Vector|MakeVector (* _index (Variables|Default|GetLength)) -1e+01 0.0) (Math|Rotator|MakeRotator 0.0 0.0 0.0) "1.000000,1.000000,1.000000")))
    (Transformation|SetRelativeScale3D _returnvalue_3 "1.500000,1.500000,1.125000"))
  (bind _returnvalue_4 (AddComponent|AddStaticMeshComponent false (Math|Transform|MakeTransform (Math|Vector|MakeVector (* (+ _returnvalue_2 1) (Variables|Default|GetLength)) -1e+01 0.0) (Math|Rotator|MakeRotator 0.0 0.0 0.0) "1.000000,1.000000,1.000000")))
  (Transformation|SetRelativeScale3D _returnvalue_4 "1.500000,1.500000,1.125000"))