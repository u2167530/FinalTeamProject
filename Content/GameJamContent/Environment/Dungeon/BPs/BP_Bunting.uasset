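; Procedural dungeon bunting that builds a sagging rope between Start and End points in the construction script.
; A three-point spline, its middle shifted by height difference and lowered by HangAmount, carries spline mesh segments cycling through five materials.
; A dynamic material receives endpoints, sag, banner colours and WPO cutoff for instanced hanging objects.
; These get random scale and spacing, though their length check passes only when usable rope is zero or less.
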(event EventBeginPlay)

(event Collision|EventActorBeginOverlap
  (params (OtherActor :type Actor%20Object%20Reference)))

(event EventTick
  (params (DeltaSeconds :type Float%20%28single-precision%29)))

(fn ConstructionScript
  ;[1 1 1] Rope Creation
  (CallFunction|SetupSpline)
  (if (and (Utilities|IsValid (Variables|Rope|GetRopeMesh)) (> (Spline|GetSplineLength (Variables|Default|GetSpline)) 1e+01))
    (CallFunction|CreateMID)
    (CallFunction|CreateRopeMesh)
    (CallFunction|SpawnHangingObjects)))

(fn SetupSpline
  (bind _end (Variables|Rope|GetEnd))
  (bind _start (Variables|Rope|GetStart))
  (bind _spline (Variables|Default|GetSpline))
  (bind _start_2 (Variables|Rope|GetStart))
  (bind _end_2 (Variables|Rope|GetEnd))
  (bind (_x _y) (Math|Vector|BreakVector _end))
  (bind (_x_2 _y_2) (Math|Vector|BreakVector _start))
  (Utilities|FlowControl|Sequence
    (:then_0
      (LocalVariables|SetMidPointDistance (+ 0.5 (Math|Float|ClampAngle (Math|Float|SafeDivide (* (- (.Z (Math|Vector|BreakVector _end)) (.Z (Math|Vector|BreakVector _start))) (LocalVariables|GetMidPointShiftScale)) (Math|Vector|Distance2D(Vector) (Math|Vector2D|MakeVector2D _x _y) (Math|Vector2D|MakeVector2D _x_2 _y_2))) -0.48 0.48))))
    (:then_1
      (LocalVariables|SetCenterPoint (Math|Vector|MakeVector (.x (+ (* (- _start_2 _end_2) (LocalVariables|GetMidPointDistance)) _end_2)) (.y (+ (* (- _start_2 _end_2) (LocalVariables|GetMidPointDistance)) _end_2)) (- (.z (+ (* (- _start_2 _end_2) (LocalVariables|GetMidPointDistance)) _end_2)) (Variables|Rope|GetHangAmount))))
      (Spline|SetSplinePoints (Variables|Default|GetSpline) (Utilities|Array|MakeArray _start_2 (Math|Vector|MakeVector (.x (+ (* (- _start_2 _end_2) (LocalVariables|GetMidPointDistance)) _end_2)) (.y (+ (* (- _start_2 _end_2) (LocalVariables|GetMidPointDistance)) _end_2)) (- (.z (+ (* (- _start_2 _end_2) (LocalVariables|GetMidPointDistance)) _end_2)) (Variables|Rope|GetHangAmount))) _end_2) "Local" true)
      ;[0.07005 1 0.2462] Tangents
      (bind _output_get (LocalVariables|SetChangeZ (Math|Float|Max(Float) (Math|Float|Absolute(Float) (- (.z (Variables|Rope|GetStart)) (.z (Variables|Rope|GetEnd)))) 1e+01)))
      (Spline|SetTangentatSplinePoint _spline 0 (Math|Vector|MakeVector 0.0 0.0 (* _output_get (LocalVariables|GetRopeHandRoundness) -1.0)) "Local" true)
      (Spline|SetTangentatSplinePoint _spline 1 (- (- (Variables|Rope|GetEnd) (Math|Vector|MakeVector 0.0 0.0 (Variables|Rope|GetHangAmount))) (LocalVariables|GetCenterPoint)) "Local" true)
      (Spline|SetTangentatSplinePoint _spline 2 (Math|Vector|MakeVector 0.0 0.0 (* (LocalVariables|GetChangeZ) (LocalVariables|GetRopeHandRoundness))) "Local" true)
      (return))))

(fn CreateMID
  (bind _returnvalue (Transformation|GetActorTransform))
  ;[1 1 1] Material Colour
  (bind _returnvalue_2 (Rendering|Material|CreateDynamicMaterialInstance "/Game/GameJamContent/Environment/Dungeon/Materials/MMI_Bunting.MMI_Bunting" "None" "Transient" :!class /Script/Engine.KismetMaterialLibrary))
  (bind _output_get (Variables|General|SetRopeMID _returnvalue_2))
  (Rendering|Material|SetVectorParameterValue _output_get "PointA" (Math|Conversions|ToLinearColor(Vector) (Math|Transform|TransformLocation _returnvalue (Variables|Rope|GetStart))) :!class /Script/Engine.MaterialInstanceDynamic)
  (Rendering|Material|SetVectorParameterValue _output_get "PointB" (Math|Conversions|ToLinearColor(Vector) (Math|Transform|TransformLocation _returnvalue (Variables|Rope|GetEnd))) :!class /Script/Engine.MaterialInstanceDynamic)
  (Rendering|Material|SetVectorParameterValue _output_get "HangAmount" (Math|Conversions|ToLinearColor(Float) (Variables|Rope|GetHangAmount)) :!class /Script/Engine.MaterialInstanceDynamic)
  ;[1 1 1] Material Colour
  (Rendering|Material|SetVectorParameterValue _output_get "BannerColour" (Variables|Colour|GetBannerColour) :!class /Script/Engine.MaterialInstanceDynamic)
  (Rendering|Material|SetScalarParameterValue _output_get "NumBannerColours" (Math|Conversions|ToFloat(Integer) (Variables|Colour|GetNumBannerColours)) :!class /Script/Engine.MaterialInstanceDynamic)
  (Rendering|Material|SetScalarParameterValue _output_get "BannerColourRandom" (Variables|Colour|GetBannerColourRandom) :!class /Script/Engine.MaterialInstanceDynamic)
  ;[1 1 1] Disabling WPO
  (Rendering|Material|SetScalarParameterValue _output_get "WPODisableDistance" (Math|Conversions|ToFloat(Integer) (Variables|General|GetWPODisableDistance)) :!class /Script/Engine.MaterialInstanceDynamic)
  (return))

(fn CreateRopeMesh
  (bind _spline (Variables|Default|GetSpline))
  (bind _ropemesh (Variables|Rope|GetRopeMesh))
  (bind _spline_2 (Variables|Default|GetSpline))
  (bind _spline_3 (Variables|Default|GetSpline))
  (bind _returnvalue (Spline|GetSplineLength _spline))
  (bind _returnvalue_2 (StaticMesh|GetBounds _ropemesh))
  (bind _returnvalue_3 (* (.x (.boxextent _returnvalue_2)) 2.0))
  (bind (_remainder _returnvalue_4) (Math|Float|Division(WholeandRemainder) _returnvalue _returnvalue_3))
  ;[1 1 1] Dividing rope into rope mesh segments
  (LocalVariables|SetSegmentWidth (+ (/ _remainder _returnvalue_4) _returnvalue_3))
  (for _index (range 0 (- _returnvalue_4 1))
    (LocalVariables|SetCurrentIndex _index)
    ;[1 0.1143 0.1342] Spawn Meshes
    (bind _returnvalue_5 (AddComponent|AddSplineMeshComponent false (Math|Transform|MakeTransform "0, 0, 0" "0, 0, 0" (Math|Vector|MakeVector 1.0 1.0 1.0))))
    (Utilities|FlowControl|Sequence
      (:then_0
        (SplineMesh|SetForwardAxis _returnvalue_5 "X" false)
        (Components|StaticMesh|SetStaticMesh _returnvalue_5 (Variables|Rope|GetMesh%20Target))
        (Collision|SetCollisionEnabled _returnvalue_5 "NoCollision")
        (Rendering|Material|SetMaterial _returnvalue_5 0 (Utilities|Array|Get(acopy) (Variables|Default|GetBuntingMaterials) (Math|Float|Truncate (.Remainder (Math|Float|Division(WholeandRemainder) (Math|Conversions|ToFloat(Integer) (LocalVariables|GetCurrentIndex)) 5.0))))))
      (:then_1
        ;[0.3664 0.9001 1] Setting mesh location and tangents
        (SplineMesh|SetStartandEnd _returnvalue_5 (Spline|GetLocationatDistanceAlongSpline _spline_3 (* (LocalVariables|GetCurrentIndex) (LocalVariables|GetSegmentWidth)) "Local") (Math|Vector|VectorClampSizeMax (Spline|GetTangentatDistanceAlongSpline _spline_3 (* (LocalVariables|GetCurrentIndex) (LocalVariables|GetSegmentWidth)) "Local") 1e+02) (Spline|GetLocationatDistanceAlongSpline _spline_2 (+ (* (LocalVariables|GetCurrentIndex) (LocalVariables|GetSegmentWidth)) (LocalVariables|GetSegmentWidth)) "Local") (Math|Vector|VectorClampSizeMax (Spline|GetTangentatDistanceAlongSpline _spline_2 (+ (* (LocalVariables|GetCurrentIndex) (LocalVariables|GetSegmentWidth)) (LocalVariables|GetSegmentWidth)) "Local") 1e+02) true :!class /Script/Engine.SplineMeshComponent)))))

(fn SpawnHangingObjects
  (bind _spline (Variables|Default|GetSpline))
  (bind _spline_2 (Variables|Default|GetSpline))
  (bind _endspawngapamount (Variables|HangingObjects|GetEndSpawnGapAmount))
  (bind _returnvalue (Spline|GetSplineLength _spline_2))
  (bind _returnvalue_2 (* _endspawngapamount 2.0))
  (bind _returnvalue_3 (- _returnvalue _returnvalue_2))
  (if (Math|Boolean|ANDBoolean (<= (Variables|HangingObjects|GetMinScale) (Variables|HangingObjects|GetMaxScale)) (<= (Variables|HangingObjects|GetMinSpacing) (Variables|HangingObjects|GetMaxSpacing)) (<= _returnvalue_3 0.0))
    ;[1 1 1] Initialize for spawn
    (LocalVariables|SetUsableRopeLength _returnvalue_3)
    (Utilities|FlowControl|Sequence
      (:then_0
        (Rendering|Material|SetMaterial (Variables|Default|GetHangingObjects) 0 (Variables|General|GetRopeMID))
        (LocalVariables|SetMeshExtentsX (.x (.boxextent (StaticMesh|GetBounds (Variables|/Script/Engine.StaticMeshComponent|GetStaticMesh (Variables|Default|GetHangingObjects)))))))
      (:then_1
        ;[1 1 1] Spawn instances
        (while (LocalVariables|GetbContinueSpawning)
          ;;[0.4393 1 0.6714] Create target spacing and scale
          (LocalVariables|SetTargetMeshSpacing (Math|Random|RandomFloatinRange (Variables|HangingObjects|GetMinSpacing) (Variables|HangingObjects|GetMaxSpacing)))
          (LocalVariables|SetTargetMeshScale (Math|Random|RandomFloatinRange (Variables|HangingObjects|GetMinScale) (Variables|HangingObjects|GetMaxScale)))
          (if (< (+ (Variables|HangingObjects|GetEndSpawnGapAmount) (LocalVariables|GetUsedRopeLength) (* (LocalVariables|GetMeshExtentsX) (LocalVariables|GetTargetMeshScale) 2.0)) (- (Spline|GetSplineLength (Variables|Default|GetSpline)) (Variables|HangingObjects|GetEndSpawnGapAmount)))
            ;[1 1 1] Spawn Mesh
            (Components|InstancedStaticMesh|AddInstance (Variables|Default|GetHangingObjects) (Math|Transform|MakeTransform (Spline|GetLocationatDistanceAlongSpline _spline (+ (Variables|HangingObjects|GetEndSpawnGapAmount) (LocalVariables|GetUsedRopeLength) (* (LocalVariables|GetMeshExtentsX) (LocalVariables|GetTargetMeshScale))) "Local") (Math|Rotator|FindLookatRotation (Spline|GetLocationatDistanceAlongSpline _spline (+ (Variables|HangingObjects|GetEndSpawnGapAmount) (LocalVariables|GetUsedRopeLength) (* (LocalVariables|GetMeshExtentsX) (LocalVariables|GetTargetMeshScale))) "Local") (+ (Spline|GetLocationatDistanceAlongSpline _spline (+ (Variables|HangingObjects|GetEndSpawnGapAmount) (LocalVariables|GetUsedRopeLength) (* (LocalVariables|GetMeshExtentsX) (LocalVariables|GetTargetMeshScale))) "Local") (Spline|GetLocationatDistanceAlongSpline _spline (+ (Variables|HangingObjects|GetEndSpawnGapAmount) (LocalVariables|GetUsedRopeLength) (* (LocalVariables|GetMeshExtentsX) (LocalVariables|GetTargetMeshScale))) "Local"))) (Math|Vector|MakeVector (LocalVariables|GetTargetMeshScale) (LocalVariables|GetTargetMeshScale) (LocalVariables|GetTargetMeshScale))) true)
            ;[1 1 1] Update used rope length
            (LocalVariables|SetUsedRopeLength (+ (LocalVariables|GetUsedRopeLength) (* (LocalVariables|GetMeshExtentsX) (LocalVariables|GetTargetMeshScale) 2.0) (LocalVariables|GetTargetMeshSpacing)))
            (else
              (LocalVariables|SetbContinueSpawning false))))
        (return)))
    (else
      (return))))