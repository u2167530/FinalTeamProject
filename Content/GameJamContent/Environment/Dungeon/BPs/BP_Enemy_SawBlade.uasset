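; BP_Enemy_SawBlade is a dungeon saw blade hazard that damages the third-person character on contact.
; Tick spins the blade around its roll axis at RotateRate.
; Hitbox overlap deals damage through a DoOnce that resets after DamageCooldown.
; It strips the inherited pawn sensing, dropable and mesh components in the construction script, and its TakeDamage always returns false, so it ignores incoming damage.
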(event OnComponentBeginOverlap(Hitbox)
  (params (OverlappedComponent :type Primitive%20Component%20Object%20Reference) (OtherActor :type Actor%20Object%20Reference) (OtherComp :type Primitive%20Component%20Object%20Reference) (OtherBodyIndex :type Integer) (bFromSweep :type Boolean) (SweepResult :type Hit%20Result%20Structure%20%28by%20ref%29))
  (bind _asbp_third_person_character (Utilities|Casting|CastToBP_ThirdPersonCharacter OtherActor))
  (Utilities|FlowControl|DoOnce false :!label _label
    (:Completed
      (Default|TakeDamage _asbp_third_person_character (Utilities|Struct|MakeS_DamageInfo (Variables|Default|GetDamage) "NewEnumerator5" "NewEnumerator0" false (Transformation|GetActorLocation)))
      (Utilities|FlowControl|Delay (Variables|Default|GetDamageCooldown))
      (goto _label Reset))))

(event EventBeginPlay
  (|CallParentFunction) ; This node is disabled and will not be called.\nDrag off pins to build functionality.
)

(event Collision|EventActorBeginOverlap
  (params (OtherActor :type Actor%20Object%20Reference))
  (|CallParentFunction OtherActor) ; This node is disabled and will not be called.\nDrag off pins to build functionality.
)

(event EventTick
  (params (DeltaSeconds :type Float%20%28single-precision%29))
  (bind _sawblade (Variables|Default|GetSawblade))
  (bind _relativerotation (Variables|/Script/Engine.SceneComponent|GetRelativeRotation _sawblade))
  (|CallParentFunction DeltaSeconds)
  (Transformation|SetRelativeRotation _sawblade (Math|Rotator|MakeRotator (+ (.roll _relativerotation) (* DeltaSeconds (* (Variables|Default|GetRotateRate) -1.0))) (.pitch _relativerotation) (.yaw _relativerotation)) false false))

(fn ConstructionScript
  (|CallParentFunction)
  (Components|DestroyComponent (Variables|Default|GetPawnSensing))
  (Components|DestroyComponent (Variables|Default|GetDropableComponent))
  (Components|DestroyComponent (Variables|Character|GetMesh)))

(fn TakeDamage
  (params (DamageInfo :type S%20Damage%20Info%20Structure))
  (return false))