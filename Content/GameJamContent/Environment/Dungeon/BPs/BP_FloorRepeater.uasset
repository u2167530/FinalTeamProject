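; BP_FloorRepeater is a dungeon floor actor that fills a rectangular area with tiled static meshes at construction time.
; Nested loops derive tile counts from Xvalue and YValue divided by Length and add a mesh component at each grid position.
; BrickOrNah sets FloorTile to brick or rock; in brick mode, each added tile gets one of three variations from an unseeded random pick, so reconstruction reshuffles them.
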(event EventBeginPlay)

(event Collision|EventActorBeginOverlap
  (params (OtherActor :type Actor%20Object%20Reference)))

(event EventTick
  (params (DeltaSeconds :type Float%20%28single-precision%29)))

(fn ConstructionScript
  (bind _length (Variables|Default|GetLength))
  (if (Variables|Default|GetBrickOrNah)
    (Components|StaticMesh|SetStaticMesh (Variables|Default|GetFloorTile) "/Game/GameJamContent/Environment/Dungeon/FBX_Models/SM_Dungeon_BrickFlooringVariation1.SM_Dungeon_BrickFlooringVariation1")
    (else
      (Components|StaticMesh|SetStaticMesh (Variables|Default|GetFloorTile) "/Game/GameJamContent/Environment/Dungeon/FBX_Models/SM_Dungeon_RockFlooring.SM_Dungeon_RockFlooring")))
  (for _index (range 0 (Math|Float|Truncate (/ (.x (Variables|Default|GetXvalue)) (Variables|Default|GetLength))))
    (for _index_2 (range 0 (Math|Float|Truncate (/ (.y (Variables|Default|GetYValue)) (Variables|Default|GetLength))))
      (if (Variables|Default|GetBrickOrNah)
        (bind _returnvalue (AddComponent|AddStaticMeshComponent false (Math|Transform|MakeTransform (Math|Vector|MakeVector (* _index _length) (* _index_2 _length) 0.0) (Math|Rotator|MakeRotator 0.0 0.0 0.0) "1.000000,1.000000,1.000000")))
        (Components|StaticMesh|SetStaticMesh _returnvalue (Utilities|Select :Index (Math|Random|RandomIntegerinRange 0 2) :Option%200 "/Game/GameJamContent/Environment/Dungeon/FBX_Models/SM_Dungeon_BrickFlooringVariation1.SM_Dungeon_BrickFlooringVariation1" :Option%201 "/Game/GameJamContent/Environment/Dungeon/FBX_Models/SM_Dungeon_BrickFlooringVariation2.SM_Dungeon_BrickFlooringVariation2" :Option%202 "/Game/GameJamContent/Environment/Dungeon/FBX_Models/SM_Dungeon_BrickFlooringVariation3.SM_Dungeon_BrickFlooringVariation3"))
        (else
          (AddComponent|AddStaticMeshComponent false (Math|Transform|MakeTransform (Math|Vector|MakeVector (* _index _length) (* _index_2 _length) 0.0) (Math|Rotator|MakeRotator 0.0 0.0 0.0) "1.000000,1.000000,1.000000")))))))