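; Dungeon turnstile with three sets of prongs and bulbs that show red when closed and green when open.
; Construction script sets bulb colour from IsClosed, and Open clears that flag, disables prong collision and turns the bulbs green.
; While open, player overlaps spin the matching prongs, with a DoOnce per trigger that resets on exit.
; A shared Spin event alternates direction via FlipFlop, using timelines to drive relative yaw.
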(event OnComponentBeginOverlap(SpinnyCollision3)
  (params (OverlappedComponent :type Primitive%20Component%20Object%20Reference) (OtherActor :type Actor%20Object%20Reference) (OtherComp :type Primitive%20Component%20Object%20Reference) (OtherBodyIndex :type Integer) (bFromSweep :type Boolean) (SweepResult :type Hit%20Result%20Structure%20%28by%20ref%29))
  (if (Utilities|DoesObjectImplementInterface OtherActor "/Game/GameJamContent/Player/BPi_Player.BPi_Player_C")
    (if (not (Variables|Default|GetIsClosed?))
      (Utilities|FlowControl|DoOnce false
        (:Completed
          (CallFunction|Spin (Variables|Default|GetSpinnyProngs3)))))))

(event OnComponentEndOverlap(SpinnyCollision3)
  (params (OverlappedComponent :type Primitive%20Component%20Object%20Reference) (OtherActor :type Actor%20Object%20Reference) (OtherComp :type Primitive%20Component%20Object%20Reference) (OtherBodyIndex :type Integer))
  (if (Utilities|DoesObjectImplementInterface OtherActor "/Game/GameJamContent/Player/BPi_Player.BPi_Player_C")
    (if (not (Variables|Default|GetIsClosed?))
      (Utilities|FlowControl|DoOnce false) ; enters at Reset
    )))

(event OnComponentBeginOverlap(SpinnyCollision1)
  (params (OverlappedComponent :type Primitive%20Component%20Object%20Reference) (OtherActor :type Actor%20Object%20Reference) (OtherComp :type Primitive%20Component%20Object%20Reference) (OtherBodyIndex :type Integer) (bFromSweep :type Boolean) (SweepResult :type Hit%20Result%20Structure%20%28by%20ref%29))
  (if (Utilities|DoesObjectImplementInterface OtherActor "/Game/GameJamContent/Player/BPi_Player.BPi_Player_C")
    (if (not (Variables|Default|GetIsClosed?))
      (Utilities|FlowControl|DoOnce false
        (:Completed
          (CallFunction|Spin (Variables|Default|GetSpinnyProngs1)))))))

(event OnComponentEndOverlap(SpinnyCollision1)
  (params (OverlappedComponent :type Primitive%20Component%20Object%20Reference) (OtherActor :type Actor%20Object%20Reference) (OtherComp :type Primitive%20Component%20Object%20Reference) (OtherBodyIndex :type Integer))
  (if (Utilities|DoesObjectImplementInterface OtherActor "/Game/GameJamContent/Player/BPi_Player.BPi_Player_C")
    (if (not (Variables|Default|GetIsClosed?))
      (Utilities|FlowControl|DoOnce false) ; enters at Reset
    )))

(event OnComponentBeginOverlap(SpinnyCollision2)
  (params (OverlappedComponent :type Primitive%20Component%20Object%20Reference) (OtherActor :type Actor%20Object%20Reference) (OtherComp :type Primitive%20Component%20Object%20Reference) (OtherBodyIndex :type Integer) (bFromSweep :type Boolean) (SweepResult :type Hit%20Result%20Structure%20%28by%20ref%29))
  (if (Utilities|DoesObjectImplementInterface OtherActor "/Game/GameJamContent/Player/BPi_Player.BPi_Player_C")
    (if (not (Variables|Default|GetIsClosed?))
      (Utilities|FlowControl|DoOnce false
        (:Completed
          (CallFunction|Spin (Variables|Default|GetSpinnyProngs2)))))))

(event OnComponentEndOverlap(SpinnyCollision2)
  (params (OverlappedComponent :type Primitive%20Component%20Object%20Reference) (OtherActor :type Actor%20Object%20Reference) (OtherComp :type Primitive%20Component%20Object%20Reference) (OtherBodyIndex :type Integer))
  (if (Utilities|DoesObjectImplementInterface OtherActor "/Game/GameJamContent/Player/BPi_Player.BPi_Player_C")
    (if (not (Variables|Default|GetIsClosed?))
      (Utilities|FlowControl|DoOnce false) ; enters at Reset
    )))

(event Custom|Spin
  (params (SpinActor :type Scene%20Component%20Object%20Reference))
  (bind _relativerotation (Variables|/Script/Engine.SceneComponent|GetRelativeRotation SpinActor))
  (bind _relativerotation_2 (Variables|/Script/Engine.SceneComponent|GetRelativeRotation SpinActor))
  (Utilities|FlowControl|FlipFlop
    (:A
      (bind _lerp (Timeline|LerpForward PlayFromStart)
        (:Update
          (Transformation|SetRelativeRotation SpinActor (Math|Rotator|Lerp(Rotator) (Math|Rotator|MakeRotator (.roll _relativerotation_2) (.pitch _relativerotation_2) (.yaw _relativerotation_2)) (Math|Rotator|MakeRotator (.roll _relativerotation_2) (.pitch _relativerotation_2) (+ (.yaw _relativerotation_2) -2e+01)) _lerp) false false))))
    (:B
      (bind _lerp_2 (Timeline|LerpBackward PlayFromStart)
        (:Update
          (Transformation|SetRelativeRotation SpinActor (Math|Rotator|Lerp(Rotator) (Math|Rotator|MakeRotator (.roll _relativerotation) (.pitch _relativerotation) (.yaw _relativerotation)) (Math|Rotator|MakeRotator (.roll _relativerotation) (.pitch _relativerotation) (+ (.yaw _relativerotation) 2e+01)) _lerp_2) false false))))))

(event Custom|Open
  (Variables|Default|SetIsClosed? false)
  (Collision|SetCollisionEnabled (Variables|Default|GetSpinnyProngs1) "NoCollision")
  (Collision|SetCollisionEnabled (Variables|Default|GetSpinnyProngs2) "NoCollision")
  (Collision|SetCollisionEnabled (Variables|Default|GetSpinnyProngs3) "NoCollision")
  (Rendering|Material|SetMaterial (Variables|Default|GetLight1) 0 "/Game/GameJamContent/Environment/Dungeon/Materials/Turnstile/Bulb/Green/MMI_TurnstileBulbGreen.MMI_TurnstileBulbGreen")
  (Rendering|Material|SetMaterial (Variables|Default|GetLight2) 0 "/Game/GameJamContent/Environment/Dungeon/Materials/Turnstile/Bulb/Green/MMI_TurnstileBulbGreen.MMI_TurnstileBulbGreen")
  (Rendering|Material|SetMaterial (Variables|Default|GetLight3) 0 "/Game/GameJamContent/Environment/Dungeon/Materials/Turnstile/Bulb/Green/MMI_TurnstileBulbGreen.MMI_TurnstileBulbGreen"))

(event EventBeginPlay
  (Components|Timeline|SetPlayRate (Variables|Default|GetLerpForward) (/ 1.0 (Variables|Default|GetSpeedInSeconds)))
  (Components|Timeline|SetPlayRate (Variables|Default|GetLerpBackward) (/ 1.0 (Variables|Default|GetSpeedInSeconds))))

(fn ConstructionScript
  (if (Variables|Default|GetIsClosed?)
    (Rendering|Material|SetMaterial (Variables|Default|GetLight1) 0 "/Game/GameJamContent/Environment/Dungeon/Materials/Turnstile/Bulb/Red/MMI_TurnstileBulbRed.MMI_TurnstileBulbRed")
    (Rendering|Material|SetMaterial (Variables|Default|GetLight2) 0 "/Game/GameJamContent/Environment/Dungeon/Materials/Turnstile/Bulb/Red/MMI_TurnstileBulbRed.MMI_TurnstileBulbRed")
    (Rendering|Material|SetMaterial (Variables|Default|GetLight3) 0 "/Game/GameJamContent/Environment/Dungeon/Materials/Turnstile/Bulb/Red/MMI_TurnstileBulbRed.MMI_TurnstileBulbRed")
    (else
      (Rendering|Material|SetMaterial (Variables|Default|GetLight1) 0 "/Game/GameJamContent/Environment/Dungeon/Materials/Turnstile/Bulb/Green/MMI_TurnstileBulbGreen.MMI_TurnstileBulbGreen")
      (Rendering|Material|SetMaterial (Variables|Default|GetLight2) 0 "/Game/GameJamContent/Environment/Dungeon/Materials/Turnstile/Bulb/Green/MMI_TurnstileBulbGreen.MMI_TurnstileBulbGreen")
      (Rendering|Material|SetMaterial (Variables|Default|GetLight3) 0 "/Game/GameJamContent/Environment/Dungeon/Materials/Turnstile/Bulb/Green/MMI_TurnstileBulbGreen.MMI_TurnstileBulbGreen"))))