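; BP_MoveableChair2 is a dungeon chair prop that implements health and damage functions, apparently meant to be knocked around when hit.
; TakeDamage only prints a debug "chair" string, and its return node is disconnected.
; An unused calculation builds a scaled vector away from the damage location with upward lift, but nothing applies it.
; The health getters and Heal return zero, and the event graph and construction script are empty.
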(event EventBeginPlay)

(event Collision|EventActorBeginOverlap
  (params (OtherActor :type Actor%20Object%20Reference)))

(event EventTick
  (params (DeltaSeconds :type Float%20%28single-precision%29)))

(fn ConstructionScript)

(fn GetCurrentHealth
  (return 0.0))

(fn GetMaxHealth
  (return 0.0))

(fn Heal
  (params (Amount :type Float%20%28double-precision%29))
  (return 0.0))

(fn TakeDamage
  (params (DamageInfo :type S%20Damage%20Info%20Structure))
  (Development|PrintString "chair"))