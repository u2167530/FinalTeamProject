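; Moveable dungeon chair that gets knocked away when it takes damage.
; TakeDamage prints a debug string, then sets CharacterMovement velocity to a fixed-speed push directly away from the damage location, and returns false.
; Health getters and Heal are stubs returning zero, so no health is tracked.
; The actor-hit handler is empty and its binding never runs.
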(event Custom|OnActorHit_Event
  (params (SelfActor :type Actor%20Object%20Reference) (OtherActor :type Actor%20Object%20Reference) (NormalImpulse :type Vector) (Hit :type Hit%20Result%20Structure%20%28by%20ref%29)))

(event EventBeginPlay)

(event Collision|EventActorBeginOverlap
  (params (OtherActor :type Actor%20Object%20Reference)))

(event EventTick
  (params (DeltaSeconds :type Float%20%28single-precision%29)))

(fn ConstructionScript)

(fn GetCurrentHealth
  (return 0.0))

(fn GetMaxHealth
  (return 0.0))

(fn Heal
  (params (Amount :type Float%20%28double-precision%29))
  (return 0.0))

(fn TakeDamage
  (params (DamageInfo :type S%20Damage%20Info%20Structure))
  (Development|PrintString "chair")
  (Variables|/Script/Engine.MovementComponent|SetVelocity (Variables|Character|GetCharacterMovement) (* (Math|Vector|Normalize (- (Transformation|GetActorLocation) (.damagelocation DamageInfo))) 2e+03))
  (return false))