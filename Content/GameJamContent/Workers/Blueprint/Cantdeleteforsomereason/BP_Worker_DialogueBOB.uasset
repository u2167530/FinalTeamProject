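; BP_Worker_DialogueBOB is a worker Blueprint for Bob that starts a dialogue when interacted with.
; Its InteractDialogue event stores the instigator, then has the ACDialogueBob component open the first conversation tree with a blank speaker name.
; The default BeginPlay, overlap and Tick events are disabled, and the construction script only calls its parent.
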(event EventBeginPlay
  (|CallParentFunction) ; This node is disabled and will not be called.\nDrag off pins to build functionality.
)

(event Collision|EventActorBeginOverlap
  (params (OtherActor :type Actor%20Object%20Reference))
  (|CallParentFunction OtherActor) ; This node is disabled and will not be called.\nDrag off pins to build functionality.
)

(event EventInteractDialogue
  (params (Instigator :type Actor%20Object%20Reference))
  (Variables|Default|SetInteractInstigator Instigator)
  (Default|OpenConversation (Variables|Default|GetAC_DialogueBob)))

(event EventTick
  (params (DeltaSeconds :type Float%20%28single-precision%29))
  (|CallParentFunction DeltaSeconds) ; This node is disabled and will not be called.\nDrag off pins to build functionality.
)

(fn ConstructionScript
  (|CallParentFunction))