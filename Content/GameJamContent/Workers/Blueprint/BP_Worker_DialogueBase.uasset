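; Base worker Blueprint for dialogue, showing the character's name as world text when the player can interact.
; Construction fills in the name and destroys the happiness meter, interact notify and dialogue box components.
; Setting the interactable state toggles the name and, when showing it, rotates it once toward the player's follow camera.
; Closing a conversation notifies the interact instigator, while the other interaction, happiness and minigame events are empty.
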(event EventBeginPlay
  (bind _asbp_third_person_character (Utilities|Casting|CastToBP_ThirdPersonCharacter (Game|GetPlayerCharacter 0)))
  (Variables|Default|SetPlayerRef _asbp_third_person_character))

(event Collision|EventActorBeginOverlap
  (params (OtherActor :type Actor%20Object%20Reference)))

(event EventSetInteractableState
  (params (ShowInteract :type Boolean))
  (bind _txt_name (Variables|Default|GetTxt_Name))
  (bind _playerref (Variables|Default|GetPlayerRef))
  (bind _returnvalue (Transformation|GetWorldLocation _txt_name))
  (bind _followcamera (Variables|/Game/GameJamContent/Player/Blueprint/BP_ThirdPersonCharacter.BP_ThirdPersonCharacter_C|GetFollowCamera _playerref))
  (bind _returnvalue_2 (Transformation|GetWorldLocation _followcamera))
  (bind _returnvalue_3 (Math|Rotator|FindLookatRotation _returnvalue _returnvalue_2))
  (if ShowInteract
    (Rendering|SetVisibility _txt_name true false)
    (Transformation|SetWorldRotation _txt_name (Math|Rotator|MakeRotator 0.0 (.pitch _returnvalue_3) (.yaw _returnvalue_3)) false false)
    (else
      (Rendering|SetVisibility (Variables|Default|GetTxt_Name) false false))))

(event EventConversationClosed
  (Class|BPiInteractableDialogue|ConversationClosed(Message) (Variables|Default|GetInteractInstigator)))

(event EventTick
  (params (DeltaSeconds :type Float%20%28single-precision%29)))

(event EventInteract)

(event EventUpdateHappiness
  (params (HappinessRate :type Float%20%28double-precision%29)))

(event EventMinigameBonus
  (params (HappinessAmount :type Float%20%28double-precision%29) (MinigameType :type E_MinigameType%20Enum :default "NewEnumerator0")))

(event EventAllowInteractions)

(event EventHoldInteract
  (params (Instigator :type Actor%20Object%20Reference)))

(event EventInteractwithObject
  (params (PlayerReference :type BP%20Third%20Person%20Character%20Object%20Reference)))

(fn ConstructionScript
  (Rendering|Components|TextRender|SetText (Variables|Default|GetTxt_Name) (Variables|Default|GetCharacterName))
  (Components|DestroyComponent (Variables|Default|GetHappinessMeter))
  (Components|DestroyComponent (Variables|Default|GetInteractNotify))
  (Components|DestroyComponent (Variables|Default|GetDialogueBox)))