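; BP_Worker is a worker whose happiness drains during a contract and is shown on a HappinessMeter widget.
; UpdateHappiness sets the drain rate, leaving the passed happiness unused, reveals the meter and starts a looping timer that lowers happiness and refreshes the widget.
; StopContract pauses that timer.
; InteractBox overlaps with BPi_Player actors toggle CanInteract, which gates GiveCoffee, currently only a debug print.
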(event OnComponentBeginOverlap(InteractBox)
  (params (OverlappedComponent :type Primitive%20Component%20Object%20Reference) (OtherActor :type Actor%20Object%20Reference) (OtherComp :type Primitive%20Component%20Object%20Reference) (OtherBodyIndex :type Integer) (bFromSweep :type Boolean) (SweepResult :type Hit%20Result%20Structure%20%28by%20ref%29))
  (if (Utilities|DoesObjectImplementInterface OtherActor "/Game/GameJamContent/Player/BPi_Player.BPi_Player_C")
    (Variables|Default|SetCanInteract true)))

(event OnComponentEndOverlap(InteractBox)
  (params (OverlappedComponent :type Primitive%20Component%20Object%20Reference) (OtherActor :type Actor%20Object%20Reference) (OtherComp :type Primitive%20Component%20Object%20Reference) (OtherBodyIndex :type Integer))
  (if (Utilities|DoesObjectImplementInterface OtherActor "/Game/GameJamContent/Player/BPi_Player.BPi_Player_C")
    (Variables|Default|SetCanInteract false)))

(event Custom|HappinessTimer
  (Variables|Default|SetHappiness (- (Variables|Default|GetHappiness) (Variables|Default|GetHappinessRate)))
  (CallFunction|UpdateHappinessUI))

(event Custom|StartContract
  (bind _returnvalue (Utilities|Time|SetTimerbyEvent (delegate Custom|HappinessTimer) 0.1 true)))

(event Custom|StopContract
  (Utilities|Time|PauseTimerbyHandle (stale Custom|StartContract _returnvalue)))

(event EventUpdateHappiness
  (params (Hapiness :type Float%20%28double-precision%29) (HappinessRate :type Float%20%28double-precision%29))
  (Variables|Default|SetHappinessRate HappinessRate)
  (Rendering|SetVisibility (Variables|Default|GetHappinessMeter) true false)
  (CallFunction|UpdateHappinessUI)
  (CallFunction|StartContract))

(event EventBeginPlay
  (CallFunction|UpdateHappinessUI))

(event EventGiveCoffee
  (if (Variables|Default|GetCanInteract)
    (Development|PrintString "Coffee Drink!!")))

(fn ConstructionScript)

(fn UpdateHappinessUI
  (Class|BPiWorkerHappinessUI|UpdateHappinessUI(Message) (UserInterface|GetWidget (Variables|Default|GetHappinessMeter)) (Variables|Default|GetHappiness)))