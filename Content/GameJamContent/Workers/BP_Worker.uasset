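; BP_Worker is a game jam worker actor that the player can give coffee to when close enough.
; Overlap events on its InteractBox set CanInteract when an actor implementing BPi_Player enters and clear it when one leaves.
; The GiveCoffee event checks that flag and, for now, only prints a debug string.
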(event OnComponentBeginOverlap(InteractBox)
  (params (OverlappedComponent :type Primitive%20Component%20Object%20Reference) (OtherActor :type Actor%20Object%20Reference) (OtherComp :type Primitive%20Component%20Object%20Reference) (OtherBodyIndex :type Integer) (bFromSweep :type Boolean) (SweepResult :type Hit%20Result%20Structure%20%28by%20ref%29))
  (if (Utilities|DoesObjectImplementInterface OtherActor "/Game/GameJamContent/Player/BPi_Player.BPi_Player_C")
    (Variables|Default|SetCanInteract true)))

(event OnComponentEndOverlap(InteractBox)
  (params (OverlappedComponent :type Primitive%20Component%20Object%20Reference) (OtherActor :type Actor%20Object%20Reference) (OtherComp :type Primitive%20Component%20Object%20Reference) (OtherBodyIndex :type Integer))
  (if (Utilities|DoesObjectImplementInterface OtherActor "/Game/GameJamContent/Player/BPi_Player.BPi_Player_C")
    (Variables|Default|SetCanInteract false)))

(event EventGiveCoffee
  (if (Variables|Default|GetCanInteract)
    (Development|PrintString "Coffee Drink!!")))

(fn ConstructionScript)